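; Sudden-death game mode for Rebound: a single tie-breaker round between the players who share the highest win count.
; Binds round-phase callbacks, shows sudden-death and end-round widgets, and starts the game on the first Tick.
; Ranks persistent wins, marking claimed scores to separate ties, then spawns leaders as pawns and configures podiums for the rest.
; AdvancePlaylist writes scores back to persistent wins and opens EndLevel or MainMenu.
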(event Custom|PostRoundCall_Copy
  (Math|Integer|IncrementInt (Variables|Default|Getround)
    (:%20%20
      (CallFunction|CheckWinConditions)
      (CallFunction|DespawnPlayerPawns))))

(event Custom|PreRoundCall_Copy
  (CallFunction|SpawnPlayerPawns))

(event Custom|StartGameCall_Copy
  (bind _gamedata (Variables|Default|GetgameData))
  (bind _aspersistent_data (Utilities|Casting|CastToPersistentData (Game|GetGameInstance)))
  (if (Variables|/Game/BluePrints/data/PersistentData.PersistentData_C|GetloadData _aspersistent_data)
    (Variables|/Game/BluePrints/data/GameData.GameData_C|SetplayerOrder _gamedata (Variables|/Game/BluePrints/data/PersistentData.PersistentData_C|GetPlayers _aspersistent_data)))
  (CallFunction|CreatePlayers (Variables|/Game/BluePrints/data/GameData.GameData_C|GetplayerOrder _gamedata)))

(event Custom|StartRoundCall_Copy
  (Variables|Default|SetLastManAliveErrorCheck -1))

(event Custom|EndRoundCall_Copy
  (Widget|SetVisibility (Variables|Default|GetEndRoundUI) "Visible"))

(event EventBeginPlay
  (CallFunction|SpawnDataActors)
  (EventDispatchers|BindEventtoStartGame (delegate Custom|StartGameCall_Copy))
  (EventDispatchers|BindEventtoStartRound (delegate Custom|StartRoundCall_Copy))
  (EventDispatchers|BindEventtoEndRound (delegate Custom|EndRoundCall_Copy))
  (EventDispatchers|BindEventtoPostRound (delegate Custom|PostRoundCall_Copy))
  (EventDispatchers|BindEventtoPreRound (delegate Custom|PreRoundCall_Copy))
  (bind _returnvalue (UserInterface|CreateWidget "/Game/UI/InGame/EndRound.EndRound_C"))
  (bind _returnvalue_2 (UserInterface|CreateWidget "/Game/UI/InGame/SuddenDeathGame.SuddenDeathGame_C"))
  (bind _output_get (Variables|Default|SetEndRoundUI _returnvalue))
  (UserInterface|Viewport|AddtoViewport _returnvalue 0)
  (Widget|SetVisibility _output_get "Hidden")
  (bind _aspersistent_data (Utilities|Casting|CastToPersistentData (Game|GetGameInstance)))
  (Variables|Default|SetPersisData _aspersistent_data)
  (Variables|Default|SetMaxRounds 1)
  (bind _outactors (Actor|GetAllActorsOfClass "/Game/BluePrints/data/SuddenDeathData.SuddenDeathData_C"))
  (Variables|Default|SetSuddenDeathData (Utilities|Array|Get(acopy) _outactors)))

(event EventAdvancePlaylist
  (bind _aspersistent_data (Utilities|Casting|CastToPersistentData (Game|GetGameInstance)))
  ;[1 1 1] set overall Scores
  (for (_array_element _array_index) (Variables|Default|GetScores)
    (Utilities|Array|SetArrayElem (Variables|/Game/BluePrints/data/PersistentData.PersistentData_C|GetWins _aspersistent_data) _array_index _array_element true))
  (if (Variables|/Game/BluePrints/data/PersistentData.PersistentData_C|GetloadData _aspersistent_data)
    ;[1 1 1] load level
    (Game|OpenLevel(byName) "EndLevel")
    (else
      ;[1 1 1] loading screen vid
      (bind _returnvalue (UserInterface|CreateWidget "/Game/UI/loadingScreen/InfoLoadingScreen.InfoLoadingScreen_C"))
      (UserInterface|Viewport|AddtoViewport _returnvalue 0)
      ;[1 1 1] load level
      (Game|OpenLevel(byName) "MainMenu"))))

(event EventTick
  (params (DeltaSeconds :type Float%20%28single-precision%29))
  (if (not (Variables|Default|GetHasStarted))
    (Default|CallStartGame)
    (Default|CallPreRound)
    (Variables|Default|SetHasStarted true)))

(event EventSpawnPlayerPawns
  (bind _scoressorted (Variables|Default|GetScoresSorted))
  (bind _tempposindex (Variables|Default|GettempPosIndex))
  (Variables|Default|SetGlobalTempScor (Variables|/Game/BluePrints/data/PersistentData.PersistentData_C|GetWins (Variables|Default|GetPersisData)))
  ;[1 1 1] set the players in ofder
  (for _index (range 0 3)
    (bind _score (CallFunction|GetScoreatRank _index))
    (bind _playernum (CallFunction|GetPlayeratScore _score))
    (Utilities|Array|Insert (Variables|Default|GetPlayerRanking) _playernum _index))
  (for (_array_element _array_index) (Variables|Default|GetPlayerRanking)
    (if (!= (Utilities|Array|Get(acopy) (Variables|/Game/BluePrints/data/GameData.GameData_C|GetplayerOrder (Variables|Default|GetgameData)) _array_element) -1)
      (if (== (.MaxValue (Math|Integer|MaxOfIntArray _scoressorted)) (Utilities|Array|Get(acopy) _scoressorted _array_index))
        (bind _asrebound_player_controller (Utilities|Casting|CastToReboundPlayerController (Game|GetPlayerController (Utilities|Array|Get(acopy) (Variables|/Game/BluePrints/data/GameData.GameData_C|GetplayerOrder (Variables|Default|GetgameData)) _array_element))))
        (Default|SpawnPawn _asrebound_player_controller (Transformation|GetActorTransform (Class|GameMode|FindPlayerStart (Game|GetPlayerController (Utilities|Array|Get(acopy) (Variables|/Game/BluePrints/data/GameData.GameData_C|GetplayerOrder (Variables|Default|GetgameData)) _array_element)))) (Variables|Default|GetMainPlayerPawn))
        (Development|PrintString "over")
        (Default|SetBlankPodium (Utilities|Array|Get(acopy) (Variables|/Game/BluePrints/data/SuddenDeathData.SuddenDeathData_C|GetPodiums (Variables|Default|GetSuddenDeathData)) _array_index))
        (elif (== (Variables|Default|GettempScoreIndex) (Utilities|Array|Get(acopy) (Variables|Default|GetScoresSorted) _array_index))
          (bind _result (Math|Integer|IncrementInt _tempposindex)
            (:%20%20
              (Default|SetUpPodium (Utilities|Array|Get(acopy) (Variables|/Game/BluePrints/data/SuddenDeathData.SuddenDeathData_C|GetPodiums (Variables|Default|GetSuddenDeathData)) _array_index) _result _array_index)))
          (else
            (Default|SetUpPodium (Utilities|Array|Get(acopy) (Variables|/Game/BluePrints/data/SuddenDeathData.SuddenDeathData_C|GetPodiums (Variables|Default|GetSuddenDeathData)) _array_index) _tempposindex _array_element)
            (Variables|Default|SettempScoreIndex (Utilities|Array|Get(acopy) (Variables|Default|GetScoresSorted) _array_index)))))
      (else
        (Rendering|SetActorHiddenInGame (Utilities|Array|Get(acopy) (Variables|/Game/BluePrints/data/SuddenDeathData.SuddenDeathData_C|GetPodiums (Variables|Default|GetSuddenDeathData)) _array_index) true))))
  (bind _outactors (Actor|GetAllActorsOfClass "/Game/BluePrints/Core-Gameplay/Characters/ReboundPlayerCharacter.ReboundPlayerCharacter_C"))
  (bind _output_get (Variables|Default|SetPlayerPawns _outactors))
  (Variables|Default|SetcurrentPlayers (- (Utilities|Array|Length _output_get) 1)))

(fn ConstructionScript
  (|CallParentFunction))

(fn GetScoreatRank
  (params (Rank :type Integer))
  (bind _output_get (LocalVariables|SetTempoaryScores (Variables|/Game/BluePrints/data/PersistentData.PersistentData_C|GetWins (Variables|Default|GetPersisData))))
  (for _index (range 0 Rank)
    (LocalVariables|SetTempScore (.MaxValue (Math|Integer|MaxOfIntArray _output_get)))
    (Utilities|Array|RemoveIndex (LocalVariables|GetTempoaryScores) (.IndexOfMaxValue (Math|Integer|MaxOfIntArray _output_get))))
  (Utilities|Array|SetArrayElem (Variables|Default|GetScoresSorted) Rank (LocalVariables|GetTempScore) true)
  (return (LocalVariables|GetTempScore)))

(fn GetPlayeratScore
  (params (Score :type Integer))
  (bind _globaltempscor (Variables|Default|GetGlobalTempScor))
  (bind _returnvalue (Utilities|Array|FindItem _globaltempscor Score))
  (bind _output_get (LocalVariables|SetTempValue _returnvalue))
  (Utilities|Array|SetArrayElem _globaltempscor _returnvalue -100)
  (return _output_get))