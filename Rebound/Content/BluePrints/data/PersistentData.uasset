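; PersistentData holds the game's graphics settings, with an Init event that creates a SaveGame_Graphics object and tries to load the saved one.
; Setter functions handle quality preset, fullscreen, resolution scale and gamma, each saving to the slot as strings.
; Quality, fullscreen and resolution apply through console commands; gamma is only stored.
; Loading restores variables without reapplying them, Init forces a fullscreen command, and a dev-mode flag controls debug messages.
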(event EventInit
  (bind _isdevmode (Variables|Default|GetisDevMode))
  (bind _returnvalue (SaveGame|CreateSaveGameObject "/Game/BluePrints/data/SaveGame_Graphics.SaveGame_Graphics_C"))
  (bind _assave_game_graphics (Utilities|Casting|CastToSaveGame_Graphics _returnvalue))
  (bind _output_get (Variables|Default|SetGraphicsInstance _assave_game_graphics))
  (bind _successful (CallFunction|LoadSettings (Variables|/Game/BluePrints/data/SaveGame_Graphics.SaveGame_Graphics_C|GetSaveSlotName _output_get)))
  (Development|ExecuteConsoleCommand "Fullscreen 2")
  (if _successful
    (Development|PrintString "Loaded" _isdevmode)
    (else
      (Development|PrintString "NotLoaded" _isdevmode)))
  (if (Variables|Default|GetisDevMode)
    (Development|ExecuteConsoleCommand "DISABLEALLSCREENMESSAGES")))

(fn OverallGraphicsChange
  (params (Graphics :type GraphicsQuality%20Enum))
  (bind _graphicsinstance (Variables|Default|GetGraphicsInstance))
  (bind _output_get (Variables|Default|SetOverallGraphicsQuality Graphics))
  (switch Utilities|FlowControl|Switch|SwitchonGraphicsQuality _output_get
    (:NewEnumerator0
      (Development|ExecuteConsoleCommand (Utilities|String|Append (Variables|graphics|GetPostProcessing) "0"))
      (Development|ExecuteConsoleCommand (Utilities|String|Append (Variables|graphics|GetShadowQuality) "1"))
      (Development|ExecuteConsoleCommand (Utilities|String|Append (Variables|graphics|GetTextureQuality) "1"))
      (Development|ExecuteConsoleCommand (Utilities|String|Append (Variables|graphics|GetEffectsQuality) "1"))
      (Development|PrintString "Graphics Set To Low" (Variables|Default|GetisDevMode))
      (Variables|/Game/BluePrints/data/SaveGame_Graphics.SaveGame_Graphics_C|SetGraphicsSetting (Variables|Default|GetGraphicsInstance) "Low"))
    (:NewEnumerator1
      (Development|ExecuteConsoleCommand (Utilities|String|Append (Variables|graphics|GetPostProcessing) "1"))
      (Development|ExecuteConsoleCommand (Utilities|String|Append (Variables|graphics|GetShadowQuality) "1"))
      (Development|ExecuteConsoleCommand (Utilities|String|Append (Variables|graphics|GetTextureQuality) "1"))
      (Development|ExecuteConsoleCommand (Utilities|String|Append (Variables|graphics|GetEffectsQuality) "1"))
      (Development|PrintString "Graphics Set To Medium" (Variables|Default|GetisDevMode))
      (Variables|/Game/BluePrints/data/SaveGame_Graphics.SaveGame_Graphics_C|SetGraphicsSetting _graphicsinstance "Medium"))
    (:NewEnumerator2
      (Development|ExecuteConsoleCommand (Utilities|String|Append (Variables|graphics|GetPostProcessing) "2"))
      (Development|ExecuteConsoleCommand (Utilities|String|Append (Variables|graphics|GetShadowQuality) "2"))
      (Development|ExecuteConsoleCommand (Utilities|String|Append (Variables|graphics|GetTextureQuality) "2"))
      (Development|ExecuteConsoleCommand (Utilities|String|Append (Variables|graphics|GetEffectsQuality) "2"))
      (Development|PrintString "Graphics Set To High" (Variables|Default|GetisDevMode))
      (Variables|/Game/BluePrints/data/SaveGame_Graphics.SaveGame_Graphics_C|SetGraphicsSetting (Variables|Default|GetGraphicsInstance) "High"))
    (:NewEnumerator3
      (Development|ExecuteConsoleCommand (Utilities|String|Append (Variables|graphics|GetPostProcessing) "3"))
      (Development|ExecuteConsoleCommand (Utilities|String|Append (Variables|graphics|GetShadowQuality) "3"))
      (Development|ExecuteConsoleCommand (Utilities|String|Append (Variables|graphics|GetTextureQuality) "3"))
      (Development|ExecuteConsoleCommand (Utilities|String|Append (Variables|graphics|GetEffectsQuality) "3"))
      (Development|PrintString "Graphics Set To Epic" (Variables|Default|GetisDevMode))
      (Variables|/Game/BluePrints/data/SaveGame_Graphics.SaveGame_Graphics_C|SetGraphicsSetting (Variables|Default|GetGraphicsInstance) "Epic")))
  (SaveGame|SaveGametoSlot _graphicsinstance (Variables|/Game/BluePrints/data/SaveGame_Graphics.SaveGame_Graphics_C|GetSaveSlotName _graphicsinstance)))

(fn FullscreenToggle
  (params (Override :type Boolean) (isFullscreen :type Boolean))
  (bind _graphicsinstance (Variables|Default|GetGraphicsInstance))
  ;[1 1 1] This is super mangled because the fullscreen console command does noes not work as expected
  (if Override
    (if isFullscreen
      (if (Variables|Default|GetisFullscreen) :!label _label
        _
        (else
          (Development|ExecuteConsoleCommand "fullscreen 2")))
      (bind _output_get (Variables|Default|SetisFullscreen true))
      (Variables|/Game/BluePrints/data/SaveGame_Graphics.SaveGame_Graphics_C|SetIsFullscreen _graphicsinstance (Utilities|String|ToString(Boolean) _output_get))
      (else
        (if (Variables|Default|GetisFullscreen) :!label _label_2
          (Development|ExecuteConsoleCommand "fullscreen 0"))
        (bind _output_get_2 (Variables|Default|SetisFullscreen false))
        (Variables|/Game/BluePrints/data/SaveGame_Graphics.SaveGame_Graphics_C|SetIsFullscreen _graphicsinstance (Utilities|String|ToString(Boolean) _output_get_2))))
    (elif (Variables|Default|GetisFullscreen)
      (goto _label_2)
      (else
        (goto _label))))
  (SaveGame|SaveGametoSlot _graphicsinstance (Variables|/Game/BluePrints/data/SaveGame_Graphics.SaveGame_Graphics_C|GetSaveSlotName _graphicsinstance)))

(fn ResolutionScale
  (params (Scale :type Integer))
  (bind _returnvalue (Math|Integer|Clamp(Integer) Scale 10 100))
  (bind _graphicsinstance (Variables|Default|GetGraphicsInstance))
  (Development|ExecuteConsoleCommand (Utilities|String|Append "r.ScreenPercentage " (Utilities|String|ToString(Integer) _returnvalue)))
  (bind _output_get (Variables|Default|SetResolutionScaleValue _returnvalue))
  (Variables|/Game/BluePrints/data/SaveGame_Graphics.SaveGame_Graphics_C|SetResolutionScale _graphicsinstance (Utilities|String|ToString(Integer) _output_get))
  (SaveGame|SaveGametoSlot _graphicsinstance (Variables|/Game/BluePrints/data/SaveGame_Graphics.SaveGame_Graphics_C|GetSaveSlotName _graphicsinstance))
  (return _returnvalue))

(fn ApplyGamma
  (params (Gamma :type Float%20%28single-precision%29))
  (bind _graphicsinstance (Variables|Default|GetGraphicsInstance))
  (bind _output_get (Variables|Default|SetGammaCorrection (Math|Float|Clamp(Float) Gamma 0.1 2.0)))
  (Variables|/Game/BluePrints/data/SaveGame_Graphics.SaveGame_Graphics_C|SetGamma _graphicsinstance (Utilities|String|ToString(Float) _output_get))
  (SaveGame|SaveGametoSlot _graphicsinstance (Variables|/Game/BluePrints/data/SaveGame_Graphics.SaveGame_Graphics_C|GetSaveSlotName _graphicsinstance)))

(fn LoadSettings
  (params (SlotName :type String))
  (bind _returnvalue (SaveGame|LoadGamefromSlot SlotName))
  (bind _assave_game_graphics (Utilities|Casting|CastToSaveGame_Graphics _returnvalue)
    (:then
      ;[1 1 1] Graphics Settings
      (switch string (Variables|/Game/BluePrints/data/SaveGame_Graphics.SaveGame_Graphics_C|GetGraphicsSetting _assave_game_graphics)
        (:Default
          (Variables|Default|SetOverallGraphicsQuality "NewEnumerator0"))
        (:Low
          (Variables|Default|SetOverallGraphicsQuality "NewEnumerator0"))
        (:Medium
          (Variables|Default|SetOverallGraphicsQuality "NewEnumerator1"))
        (:High
          (Variables|Default|SetOverallGraphicsQuality "NewEnumerator2"))
        (:Epic
          (Variables|Default|SetOverallGraphicsQuality "NewEnumerator3")))
      (Variables|Default|SetGammaCorrection (Math|Conversions|ToFloat(Integer) (Variables|/Game/BluePrints/data/SaveGame_Graphics.SaveGame_Graphics_C|GetGamma _assave_game_graphics)))
      (Variables|Default|SetResolutionScaleValue (Math|Conversions|ToInteger(Byte) (Variables|/Game/BluePrints/data/SaveGame_Graphics.SaveGame_Graphics_C|GetResolutionScale _assave_game_graphics)))
      (switch string (Variables|/Game/BluePrints/data/SaveGame_Graphics.SaveGame_Graphics_C|GetIsFullscreen _assave_game_graphics)
        (:Default
          _)
        (:true
          (Variables|Default|SetisFullscreen true))
        (:false
          (Variables|Default|SetisFullscreen false)))
      (Variables|Default|SetGraphicsInstance _assave_game_graphics)
      (Variables|Default|SetSettingsLoaded true)
      (return true))
    (:CastFailed
      (return false))))

(fn ToggleDevMode
  (bind _output_get (Variables|Default|SetisDevMode (not (Variables|Default|GetisDevMode))))
  (if _output_get
    (Development|ExecuteConsoleCommand "DISABLEALLSCREENMESSAGES")
    (Development|PrintString "enable")
    (else
      (Development|ExecuteConsoleCommand "ENABLEALLSCREENMESSAGES")
      (Development|PrintString "disable Dev Mode"))))