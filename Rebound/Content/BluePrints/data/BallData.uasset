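; Manages the dodgeball population during rounds, spawning balls at active Ballspawn points and clearing them at round end.
; ReboundGameMode round events trigger a shuffled initial spawn or full despawn and toggle Inplay.
; While in play, Tick tops BallCount up to BallToSpawn, preferring a random unobstructed point, then the first free one, then any random one.
; DestroyABall decrements the count only for starter balls, so only those get replaced.
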(event Custom|StartRoundCall
  (CallFunction|SpawnBalls)
  (Variables|Default|SetInplay true))

(event Custom|EndRoundCall
  (CallFunction|DespawnBalls)
  (Variables|Default|SetInplay false))

(event EventBeginPlay
  (bind _aspersistent_data (Utilities|Casting|CastToPersistentData (Game|GetGameInstance)))
  (Variables|Default|SetpersisData _aspersistent_data)
  (CallFunction|GetBallSpawns)
  (bind _asrebound_game_mode (Utilities|Casting|CastToReboundGameMode (Game|GetGameMode)))
  (EventDispatchers|BindEventtoStartRound _asrebound_game_mode (delegate Custom|StartRoundCall))
  (EventDispatchers|BindEventtoEndRound _asrebound_game_mode (delegate Custom|EndRoundCall)))

(event EventTick
  (params (DeltaSeconds :type Float%20%28single-precision%29))
  (if (Variables|Default|GetInplay)
    (if (< (Variables|Default|GetBallCount) (Variables|Default|GetBallToSpawn))
      (bind _asrebound_game_mode (Utilities|Casting|CastToReboundGameMode (Game|GetGameMode)))
      (CallFunction|SpawnABall (Variables|/Game/BluePrints/Gamemodes/ReboundGameMode.ReboundGameMode_C|GetMainDodgeBall _asrebound_game_mode) false)
      (Development|PrintString "respawn ball" (Variables|/Game/BluePrints/data/PersistentData.PersistentData_C|GetisDevMode (Variables|Default|GetpersisData))))))

(fn ConstructionScript)

(fn GetBallSpawns
  (bind _outactors (Actor|GetAllActorsOfClass "/Game/BluePrints/Core-Gameplay/Ballspawn.Ballspawn_C"))
  (for _array_element _outactors
    (if (Variables|/Game/BluePrints/Core-Gameplay/Ballspawn.Ballspawn_C|GetisActive _array_element)
      (Utilities|Array|AddUnique (Variables|Default|GetBallSpawns) _array_element)))
  (Development|PrintString "Ball Spawns" (Variables|/Game/BluePrints/data/PersistentData.PersistentData_C|GetisDevMode (Variables|Default|GetpersisData))))

(fn SpawnBalls
  (bind _ballspawns (Variables|Default|GetBallSpawns))
  (bind _asrebound_game_mode (Utilities|Casting|CastToReboundGameMode (Game|GetGameMode)))
  (Utilities|Array|Shuffle _ballspawns)
  (for _array_element _ballspawns
    (if (not (>= (Variables|Default|GetBallCount) (Variables|Default|GetBallToSpawn)))
      (bind _returnvalue (Game|SpawnActorfromClass (Variables|/Game/BluePrints/Gamemodes/ReboundGameMode.ReboundGameMode_C|GetMainDodgeBall _asrebound_game_mode) (Math|Transform|MakeTransform (Variables|/Game/BluePrints/Core-Gameplay/Ballspawn.Ballspawn_C|GetSpawnLocation _array_element) "0, 0, 0" "1,1,1") "AdjustIfPossibleButDontSpawnIfColliding" 0 0))
      (Utilities|IsValid _returnvalue
        (:Is%20Valid
          (Math|Integer|IncrementInt (Variables|Default|GetBallCount)))))))

(fn DespawnBalls
  (bind _outactors (Actor|GetAllActorsOfClass "/Game/BluePrints/Core-Gameplay/Dodgeballs/DodgeBall.DodgeBall_C"))
  (for _array_element _outactors
    (Actor|DestroyActor _array_element))
  (Variables|Default|SetBallCount 0)
  (Default|CallBallDestroyed))

(fn SpawnABall
  (params (BallType :type Dodge%20Ball%20Class%20Reference) (InitialSpawn :type Boolean))
  (bind _ballspawns (Variables|Default|GetBallSpawns))
  (bind _returnvalue (Utilities|Array|Length _ballspawns))
  (bind _returnvalue_2 (Math|Random|RandomInteger _returnvalue))
  (bind _item (Utilities|Array|Get(acopy) _ballspawns _returnvalue_2))
  (bind _output_get (LocalVariables|SetTempSpawn _item))
  (if (Variables|/Game/BluePrints/Core-Gameplay/Ballspawn.Ballspawn_C|GetIsObstructed _output_get)
    (for _array_element _ballspawns
      (if (not (LocalVariables|GetFoundEmptySpawn))
        (if (not (Variables|/Game/BluePrints/Core-Gameplay/Ballspawn.Ballspawn_C|GetIsObstructed _array_element))
          (LocalVariables|SetFoundEmptySpawn true)
          (LocalVariables|SetTempSpawn _array_element))))
    (if (LocalVariables|GetFoundEmptySpawn)
      (bind _returnvalue_3 (Game|SpawnActorfromClass BallType (Math|Transform|MakeTransform (Variables|/Game/BluePrints/Core-Gameplay/Ballspawn.Ballspawn_C|GetSpawnLocation (LocalVariables|GetTempSpawn)) "0, 0, 0" "1,1,1") "AlwaysSpawn" 0 0))
      (if (!= _returnvalue_3 0)
        (Development|PrintString "find first empty spawn" (Variables|/Game/BluePrints/data/PersistentData.PersistentData_C|GetisDevMode (Variables|Default|GetpersisData)) true "(R=1.000000,G=0.484746,B=0.006370,A=1.000000)")
        (Math|Integer|IncrementInt (Variables|Default|GetBallCount) :!label _label))
      (else
        (bind _output_get_2 (LocalVariables|SetTempSpawn _item))
        (bind _returnvalue_4 (Game|SpawnActorfromClass BallType (Math|Transform|MakeTransform (Variables|/Game/BluePrints/Core-Gameplay/Ballspawn.Ballspawn_C|GetSpawnLocation _output_get_2) "0, 0, 0" "1,1,1") "AlwaysSpawn" 0 0))
        (if (!= _returnvalue_4 0)
          (Development|PrintString "Random Spawn" (Variables|/Game/BluePrints/data/PersistentData.PersistentData_C|GetisDevMode (Variables|Default|GetpersisData)) true "(R=1.000000,G=0.638169,B=0.000000,A=1.000000)")
          (goto _label))))
    (else
      (bind _returnvalue_5 (Game|SpawnActorfromClass BallType (Math|Transform|MakeTransform (Variables|/Game/BluePrints/Core-Gameplay/Ballspawn.Ballspawn_C|GetSpawnLocation _output_get) "0, 0, 0" "1,1,1") "AlwaysSpawn" 0 0))
      (if (!= _returnvalue_5 0)
        (Development|PrintString "Inital Random Spawn" (Variables|/Game/BluePrints/data/PersistentData.PersistentData_C|GetisDevMode (Variables|Default|GetpersisData)) true "(R=1.000000,G=0.538962,B=0.172655,A=1.000000)")
        (goto _label)))))

(fn DestroyABall
  (params (BallDestroy :type Dodge%20Ball%20Object%20Reference))
  (bind _ballcount (Variables|Default|GetBallCount))
  (if (Variables|/Game/BluePrints/Core-Gameplay/Dodgeballs/DodgeBall.DodgeBall_C|GetStarterBall BallDestroy)
    (Actor|DestroyActor BallDestroy)
    (Math|Integer|DecrementInt _ballcount
      (:%20%20
        (Development|PrintString (Utilities|String|Append "Ball Destryed, Balls left: " (Utilities|String|ToString(Integer) _ballcount)) (Variables|/Game/BluePrints/data/PersistentData.PersistentData_C|GetisDevMode (Variables|Default|GetpersisData)))
        (Default|CallBallDestroyed)))
    (else
      (Actor|DestroyActor BallDestroy))))