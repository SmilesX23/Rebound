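; Fire hazard actor that burns the fireball player character while it stands inside its sphere trigger.
; On overlap begin it calls EnterFire on the character, passing a fire factor and a time-to-die value.
; On overlap end it calls ExitFire with a burn time.
; The actor destroys itself after a configurable lifetime set on BeginPlay.
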(event OnComponentBeginOverlap(Sphere)
  (params (OtherActor :type Actor%20Object%20Reference) (OtherComp :type Primitive%20Component%20Object%20Reference) (OtherBodyIndex :type Integer) (bFromSweep :type Boolean) (SweepResult :type Hit%20Result%20Structure%20%28by%20ref%29))
  (bind _asrebound_player_character_fire_ball (Utilities|Casting|CastToReboundPlayerCharacter_FireBall OtherActor))
  (Default|EnterFire _asrebound_player_character_fire_ball (Variables|Default|GetonFireFactor) (Variables|Default|GetOnFireToDie)))

(event OnComponentEndOverlap(Sphere)
  (params (OtherActor :type Actor%20Object%20Reference) (OtherComp :type Primitive%20Component%20Object%20Reference) (OtherBodyIndex :type Integer))
  (bind _asrebound_player_character_fire_ball (Utilities|Casting|CastToReboundPlayerCharacter_FireBall OtherActor))
  (Default|ExitFire _asrebound_player_character_fire_ball (Variables|Default|GetBurnTime)))

(event EventBeginPlay
  (Actor|SetLifeSpan (Variables|Default|GetLifeTime)))

(fn ConstructionScript)