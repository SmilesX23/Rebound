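; Main menu game mode for Rebound that runs the menu screens, local four-player lobby and match launch.
; BeginPlay creates every menu widget up front; ShowMenu toggles visibility, and controller input routes to the current menu.
; Tick rotates the backdrop or, in the lobby, polls each controller for joining and readying.
; StartGame writes players and a quick, custom or premade playlist into PersistentData, then loads the first level.
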(event Custom|UpUI
  (switch Utilities|FlowControl|Switch|SwitchonMenuViews (Variables|Default|GetCurrentMenu)
    (:NewEnumerator0
      (Default|UpUI (Variables|Default|GetmainMenu)))
    (:NewEnumerator1
      (Default|UpUI (Variables|Default|GetlobbyMenu)))
    (:NewEnumerator2
      (Default|UpUI (Variables|Default|GetOptionsMenu)))
    (:NewEnumerator3
      (Default|UpUI (Variables|Default|GetStreamMenu)))
    (:NewEnumerator4
      (Default|UpUI (Variables|Default|GetcustomMenu)))
    (:NewEnumerator5
      (Default|UpUI (Variables|Default|GetonlineMenu)))))

(event Custom|DownUI
  (switch Utilities|FlowControl|Switch|SwitchonMenuViews (Variables|Default|GetCurrentMenu)
    (:NewEnumerator0
      (Default|DownUI (Variables|Default|GetmainMenu)))
    (:NewEnumerator1
      (Default|DownUI (Variables|Default|GetlobbyMenu)))
    (:NewEnumerator2
      (Default|DownUI (Variables|Default|GetOptionsMenu)))
    (:NewEnumerator3
      (Default|DownUI (Variables|Default|GetStreamMenu)))
    (:NewEnumerator4
      (Default|DownUI (Variables|Default|GetcustomMenu)))
    (:NewEnumerator5
      (Default|DownUI (Variables|Default|GetonlineMenu)))))

(event Custom|load%20level
  (params (name :type Name))
  (Utilities|FlowControl|Delay 5.0)
  (Game|OpenLevel(byName) name))

(event Custom|ConfirmUI
  (switch Utilities|FlowControl|Switch|SwitchonMenuViews (Variables|Default|GetCurrentMenu)
    (:NewEnumerator0
      (Default|SelectUI (Variables|Default|GetmainMenu)))
    (:NewEnumerator1
      (Default|SelectUI (Variables|Default|GetlobbyMenu)))
    (:NewEnumerator2
      (Default|SelectUI (Variables|Default|GetOptionsMenu)))
    (:NewEnumerator3
      (Default|SelectUI (Variables|Default|GetStreamMenu)))
    (:NewEnumerator4
      (Default|SelectUI (Variables|Default|GetcustomMenu)))
    (:NewEnumerator5
      (Default|SelectUI (Variables|Default|GetonlineMenu)))))

(event Custom|ExitUI
  (switch Utilities|FlowControl|Switch|SwitchonMenuViews (Variables|Default|GetCurrentMenu)
    (:NewEnumerator1
      (Default|BackEvent (Variables|Default|GetlobbyMenu)))
    (:NewEnumerator2
      (Default|BackButton (Variables|Default|GetOptionsMenu)))
    (:NewEnumerator4
      (Default|BackButton (Variables|Default|GetcustomMenu)))))

(event Custom|LeftUI
  (switch Utilities|FlowControl|Switch|SwitchonMenuViews (Variables|Default|GetCurrentMenu)
    (:NewEnumerator1
      (Default|MoveUIFocusRight (Variables|Default|GetlobbyMenu)))
    (:NewEnumerator2
      (Default|Switch (Variables|Default|GetOptionsMenu) true))
    (:NewEnumerator4
      (Default|MoveUIFocusRight (Variables|Default|GetcustomMenu)))
    (:NewEnumerator5
      (Default|MoveUIFocusRight (Variables|Default|GetonlineMenu)))))

(event Custom|RightUI
  (switch Utilities|FlowControl|Switch|SwitchonMenuViews (Variables|Default|GetCurrentMenu)
    (:NewEnumerator1
      (Default|MoveUIFocusLeft (Variables|Default|GetlobbyMenu)))
    (:NewEnumerator2
      (Default|Switch (Variables|Default|GetOptionsMenu) false))
    (:NewEnumerator4
      (Default|MoveUIFocusLeft (Variables|Default|GetcustomMenu)))
    (:NewEnumerator5
      (Default|MoveUIFocusLeft (Variables|Default|GetonlineMenu)))))

(event EventBeginPlay
  (Utilities|FlowControl|Sequence
    (:then_0
      ;[0.1154 1 0] main menu
      (bind _returnvalue (UserInterface|CreateWidget "/Game/UI/MainMenu/MainMenu.MainMenu_C" (Game|GetPlayerController 0)))
      (bind _output_get (Variables|Default|SetmainMenu _returnvalue))
      (UserInterface|Viewport|AddtoViewport _output_get 0)
      (Widget|SetVisibility _output_get "Visible")
      (Variables|Default|SetCurrentMenu "NewEnumerator0"))
    (:then_1
      ;[1 0.455 0] quickplay
      (bind _returnvalue_2 (UserInterface|CreateWidget "/Game/UI/MainMenu/MainMenuLobby.MainMenuLobby_C" (Game|GetPlayerController 0)))
      (bind _output_get_2 (Variables|Default|SetlobbyMenu _returnvalue_2))
      (UserInterface|Viewport|AddtoViewport _output_get_2 0)
      (Widget|SetVisibility _output_get_2 "Hidden"))
    (:then_2
      ;[0.04938 0 1] options menu
      (bind _returnvalue_3 (UserInterface|CreateWidget "/Game/UI/MainMenu/MainMenuOptions.MainMenuOptions_C" (Game|GetPlayerController 0)))
      (bind _output_get_3 (Variables|Default|SetOptionsMenu _returnvalue_3))
      (UserInterface|Viewport|AddtoViewport _output_get_3 0)
      (Widget|SetVisibility _output_get_3 "Hidden"))
    (:then_3
      ;[1 0.9945 0] stream menu
      (bind _returnvalue_4 (UserInterface|CreateWidget "/Game/UI/MainMenu/MainMenuLiveStream.MainMenuLiveStream_C" (Game|GetPlayerController 0)))
      (bind _output_get_4 (Variables|Default|SetStreamMenu _returnvalue_4))
      (UserInterface|Viewport|AddtoViewport _output_get_4 0)
      (Widget|SetVisibility _output_get_4 "Hidden"))
    (:then_4
      ;[1 0 0.4665] custom playlist menu
      (bind _returnvalue_5 (UserInterface|CreateWidget "/Game/UI/MainMenu/MainMenuCustomPlaylist.MainMenuCustomPlaylist_C" (Game|GetPlayerController 0)))
      (bind _output_get_5 (Variables|Default|SetcustomMenu _returnvalue_5))
      (UserInterface|Viewport|AddtoViewport _output_get_5 0)
      (Widget|SetVisibility _output_get_5 "Hidden"))
    (:then_5
      ;[0 0.8635 1] custom playlist menu
      (bind _returnvalue_6 (UserInterface|CreateWidget "/Game/UI/MainMenu/OnlineMenu.OnlineMenu_C" (Game|GetPlayerController 0)))
      (bind _output_get_6 (Variables|Default|SetonlineMenu _returnvalue_6))
      (UserInterface|Viewport|AddtoViewport _output_get_6 0)
      (Widget|SetVisibility _output_get_6 "Hidden"))
    (:then_6
      (bind _asnetworking_player_controller (Utilities|Casting|CastToNetworkingPlayerController (Game|GetPlayerController 0)))
      (EventDispatchers|BindEventtoButtonUp _asnetworking_player_controller (delegate Custom|UpUI))
      (EventDispatchers|BindEventtoButtonDown _asnetworking_player_controller (delegate Custom|DownUI))
      (EventDispatchers|AssignButtonConfirm _asnetworking_player_controller (delegate Custom|ConfirmUI))
      (EventDispatchers|AssignButtonEscape _asnetworking_player_controller (delegate Custom|ExitUI))
      (EventDispatchers|AssignButtonLeft _asnetworking_player_controller (delegate Custom|LeftUI))
      (EventDispatchers|AssignButtonRight _asnetworking_player_controller (delegate Custom|RightUI)))
    (:then_7
      (CallFunction|CreatePlayers)
      ;[1 1 1] show mouse
      (Variables|/Script/Engine.PlayerController|SetbShowMouseCursor (Game|GetPlayerController 0) true)
      (bind _outactors (Actor|GetAllActorsOfClass "/Game/UI/MainMenu/MainMenuBP.MainMenuBP_C"))
      (Variables|Default|Setenviro (Variables|/Game/UI/MainMenu/MainMenuBP.MainMenuBP_C|Getenviroment (Utilities|Array|Get(acopy) _outactors)))
      (Variables|Default|Setmatinee (Variables|/Game/UI/MainMenu/MainMenuBP.MainMenuBP_C|Getmatinee (Utilities|Array|Get(acopy) _outactors)))
      (Variables|Default|Setfloor (Variables|/Game/UI/MainMenu/MainMenuBP.MainMenuBP_C|Getfloor (Utilities|Array|Get(acopy) _outactors)))
      (Game|Player|SetViewTargetwithBlend (Game|GetPlayerController 0) (Variables|/Game/UI/MainMenu/MainMenuBP.MainMenuBP_C|Getcamera (Utilities|Array|Get(acopy) _outactors)) 0.0 "VTBlend_Linear" 0.0 false)
      (bind _aspersistent_data (Utilities|Casting|CastToPersistentData (Game|GetGameInstance)))
      (Variables|Default|SetPersisData _aspersistent_data))))

(event EventTick
  (params (DeltaSeconds :type Float%20%28single-precision%29))
  (bind _rotationspeed (Variables|Default|GetrotationSpeed))
  (bind _returnvalue (* _rotationspeed DeltaSeconds))
  (switch Utilities|FlowControl|Switch|SwitchonMenuViews (Variables|Default|GetCurrentMenu)
    (:NewEnumerator0
      ;[1 1 1] rotate background
      (Class|Actor|AddActorWorldRotation (Variables|Default|Getenviro) (Math|Rotator|MakeRotator 0.0 0.0 _returnvalue) :!label _label)
      (Class|Actor|AddActorWorldRotation (Variables|Default|Getfloor) (Math|Rotator|MakeRotator 0.0 0.0 _returnvalue)))
    (:NewEnumerator1
      ;[1 1 1] lobby loop
      (CallFunction|CheckforNewPlayers)
      (CallFunction|CheckforReady))
    (:NewEnumerator2
      (goto _label))
    (:NewEnumerator3
      (goto _label))
    (:NewEnumerator5
      (goto _label))))

(event Input|ActionEvents|InputActionUpUI
  (params (Key :type Key%20Structure :default "AnyKey")))

(event Input|ActionEvents|InputActionSelectUI
  (params (Key :type Key%20Structure :default "AnyKey")))

(event Input|ActionEvents|InputActionDownUI
  (params (Key :type Key%20Structure :default "AnyKey")))

(event Input|ActionEvents|InputActionswapUIleft
  (params (Key :type Key%20Structure :default "AnyKey")))

(event Input|ActionEvents|InputActionswapUIRight
  (params (Key :type Key%20Structure :default "AnyKey")))

(event Input|ActionEvents|InputActionExit
  (params (Key :type Key%20Structure :default "AnyKey")))

(fn ConstructionScript)

(fn CreatePlayers)

(fn CheckforNewPlayers
  (if (not (Variables|/Game/UI/MainMenu/MainMenuLobby.MainMenuLobby_C|GetEnableButtons (Variables|Default|GetlobbyMenu)))
    (for _index (range 0 3)
      (if (and (or (Game|Player|WasInputKeyJustPressed (Game|GetPlayerController _index) "Gamepad_FaceButton_Left") (Game|Player|WasInputKeyJustPressed (Game|GetPlayerController _index) "SpaceBar")) (not (Utilities|Array|Get(acopy) (Variables|Default|GetplayerActiveArray) _index)))
        (Utilities|Array|SetArrayElem (Variables|Default|GetPlayerOrder) _index _index true)
        (Utilities|Array|SetArrayElem (Variables|Default|GetplayerActiveArray) _index true)
        (Default|CallPlayerAdded _index)
        (Development|PrintString (Utilities|String|BuildString(Integer) "" "player" _index "added") (Variables|/Game/BluePrints/data/PersistentData.PersistentData_C|GetisDevMode (Variables|Default|GetpersisData)))))))

(fn CheckforRemovePlayer
  (bind _playerorder (Variables|Default|GetPlayerOrder))
  (if (not (Variables|/Game/UI/MainMenu/MainMenuLobby.MainMenuLobby_C|GetEnableButtons (Variables|Default|GetlobbyMenu)))
    (for _index (range 0 3)
      (if (and (Game|Player|WasInputKeyJustPressed (Game|GetPlayerController _index) "Gamepad_FaceButton_Left") (and (Utilities|Array|Get(acopy) (Variables|Default|GetplayerActiveArray) _index) (Utilities|Array|Get(acopy) (Variables|Default|GetplayerActiveLastFrame) _index)))
        (Default|CallPlayerRemoved (Utilities|Array|FindItem _playerorder _index))
        (Variables|Default|SetcurPlayerID (Utilities|Array|FindItem _playerorder _index))
        (Utilities|Array|SetArrayElem _playerorder (Utilities|Array|FindItem _playerorder _index) -1)
        (Utilities|Array|SetArrayElem (Variables|Default|GetplayerActiveArray) _index false)
        (Utilities|Array|SetArrayElem (Variables|Default|GetplayerReadyArray) _index false)
        (Default|CallPlayerReady (Variables|Default|GetcurPlayerID) false)
        (Development|PrintString (Utilities|String|BuildString(Integer) "" "player" _index "removed") (Variables|/Game/BluePrints/data/PersistentData.PersistentData_C|GetisDevMode (Variables|Default|GetpersisData)))))
    (Variables|Default|SetplayerActiveLastFrame (Variables|Default|GetplayerActiveArray))))

(fn StartGame
  (params (Type :type PlaylistType%20Enum))
  (bind _lobbymenu (Variables|Default|GetlobbyMenu))
  (bind _playerorder (Variables|Default|GetPlayerOrder))
  (bind _aspersistent_data (Utilities|Casting|CastToPersistentData (Game|GetGameInstance)))
  ;[1 1 1] clear old data
  (Utilities|Array|Clear (Variables|/Game/BluePrints/data/PersistentData.PersistentData_C|GetWins _aspersistent_data))
  (Utilities|Array|Clear (Variables|/Game/BluePrints/data/PersistentData.PersistentData_C|GetLevelList _aspersistent_data))
  (Utilities|Array|Clear (Variables|/Game/BluePrints/data/PersistentData.PersistentData_C|GetMutatorsList _aspersistent_data))
  (Utilities|Array|Clear (Variables|/Game/BluePrints/data/PersistentData.PersistentData_C|GetPlayers _aspersistent_data))
  (Utilities|Array|Clear (Variables|/Game/BluePrints/data/PersistentData.PersistentData_C|Getrounds _aspersistent_data))
  (Utilities|Array|Clear (Variables|/Game/BluePrints/data/PersistentData.PersistentData_C|GetlevelsEnum _aspersistent_data))
  (switch Utilities|FlowControl|Switch|SwitchonPlaylistType Type
    (:NewEnumerator0
      ;[1 1 1] quick play
      (bind _outactors (Actor|GetAllActorsOfClass "/Game/UI/MainMenu/MainMenuBP.MainMenuBP_C"))
      (Utilities|Array|Shuffle (Variables|/Game/UI/MainMenu/MainMenuBP.MainMenuBP_C|Getlevels (Utilities|Array|Get(acopy) _outactors)))
      (Utilities|Array|Resize (Variables|/Game/UI/MainMenu/MainMenuBP.MainMenuBP_C|Getlevels (Utilities|Array|Get(acopy) _outactors)) 5)
      (Variables|/Game/BluePrints/data/PersistentData.PersistentData_C|SetLevelList _aspersistent_data (Variables|/Game/UI/MainMenu/MainMenuBP.MainMenuBP_C|Getlevels (Utilities|Array|Get(acopy) _outactors)))
      (Utilities|Array|Shuffle (Variables|/Game/UI/MainMenu/MainMenuBP.MainMenuBP_C|GetMutators (Utilities|Array|Get(acopy) _outactors)))
      (Utilities|Array|Resize (Variables|/Game/UI/MainMenu/MainMenuBP.MainMenuBP_C|GetMutators (Utilities|Array|Get(acopy) _outactors)) 5)
      (Variables|/Game/BluePrints/data/PersistentData.PersistentData_C|SetMutatorsList _aspersistent_data (Variables|/Game/UI/MainMenu/MainMenuBP.MainMenuBP_C|GetMutators (Utilities|Array|Get(acopy) _outactors)))
      (Variables|/Game/BluePrints/data/PersistentData.PersistentData_C|Setrounds _aspersistent_data (Utilities|Array|MakeArray 5 5 5 5 5)))
    (:NewEnumerator1
      ;[1 1 1] custom
      (Default|SetCustomPlaylist (Variables|Default|GetcustomMenu))
      (Development|PrintString "custom playlist " (Variables|/Game/BluePrints/data/PersistentData.PersistentData_C|GetisDevMode (Variables|Default|GetpersisData)) true "(R=1.000000,G=1.000000,B=1.000000,A=1.000000)" 1e+01))
    (:NewEnumerator2
      ;[1 1 1] playlist
      (Variables|/Game/BluePrints/data/PersistentData.PersistentData_C|SetLevelList _aspersistent_data (Variables|/Game/UI/MainMenu/MainMenuLobby.MainMenuLobby_C|GetlevelList _lobbymenu))
      (Variables|/Game/BluePrints/data/PersistentData.PersistentData_C|SetMutatorsList _aspersistent_data (Variables|/Game/UI/MainMenu/MainMenuLobby.MainMenuLobby_C|GetMutatorsList _lobbymenu))
      (Variables|/Game/BluePrints/data/PersistentData.PersistentData_C|Setrounds _aspersistent_data (Variables|/Game/UI/MainMenu/MainMenuLobby.MainMenuLobby_C|GetRoundsList _lobbymenu))))
  ;[1 1 1] setplayer order
  (Variables|/Game/BluePrints/data/PersistentData.PersistentData_C|SetplaylistID _aspersistent_data 0)
  (Variables|/Game/BluePrints/data/PersistentData.PersistentData_C|SetloadData _aspersistent_data true)
  (Variables|/Game/BluePrints/data/PersistentData.PersistentData_C|SetPlayers _aspersistent_data _playerorder)
  (for (_array_element _array_index) _playerorder
    (Development|PrintString (Utilities|String|BuildString(Integer) (Utilities|String|BuildString(Integer) "" "player pos" _array_index "contains ") "player ID" _array_element) (Variables|/Game/BluePrints/data/PersistentData.PersistentData_C|GetisDevMode (Variables|Default|GetpersisData))))
  (Default|CallAllPlayersReady)
  (bind _foundwidgets (Widget|GetAllWidgetsOfClass "/Game/UI/MainMenu/MainMenuLobby.MainMenuLobby_C" true))
  (Widget|SetVisibility (Utilities|Array|Get(acopy) _foundwidgets) "Hidden")
  ;[1 1 1] loading screen vid
  (bind _returnvalue (UserInterface|CreateWidget "/Game/UI/loadingScreen/InfoLoadingScreen.InfoLoadingScreen_C"))
  (UserInterface|Viewport|AddtoViewport _returnvalue 0)
  (CallFunction|LoadLevel (Utilities|Array|Get(acopy) (Variables|/Game/BluePrints/data/PersistentData.PersistentData_C|GetLevelList _aspersistent_data))))

(fn CheckforReady
  (bind _playerreadyarray (Variables|Default|GetplayerReadyArray))
  (bind _lobbymenu (Variables|Default|GetlobbyMenu))
  (if (not (Variables|/Game/UI/MainMenu/MainMenuLobby.MainMenuLobby_C|GetEnableButtons (Variables|Default|GetlobbyMenu)))
    (for _index (range 0 3)
      (if (and (or (Game|Player|WasInputKeyJustPressed (Game|GetPlayerController _index) "Gamepad_FaceButton_Top") (Game|Player|WasInputKeyJustPressed (Game|GetPlayerController _index) "Enter")) (Utilities|Array|Get(acopy) (Variables|Default|GetplayerActiveArray) _index))
        (Default|CallPlayerReady (Utilities|Array|FindItem (Variables|Default|GetPlayerOrder) _index) (not (Utilities|Array|Get(acopy) _playerreadyarray _index)))
        (Utilities|Array|SetArrayElem _playerreadyarray _index (not (Utilities|Array|Get(acopy) _playerreadyarray _index)))))
    (bind (_array_element _array_index) (Utilities|Array|ForEachLoopwithBreak (Variables|Default|GetplayerActiveArray) :!label _label)
      (:LoopBody
        (if _array_element
          (if (Utilities|Array|Get(acopy) (Variables|Default|GetplayerReadyArray) _array_index)
            (LocalVariables|Setplay true)
            (else
              (LocalVariables|Setplay false)
              (goto _label Break)))))
      (:Completed
        (if (LocalVariables|Getplay)
          (Widget|SetVisibility (Variables|/Game/UI/MainMenu/MainMenuLobby.MainMenuLobby_C|GetButtonsBox _lobbymenu) "Visible")
          (Widget|SetVisibility (Variables|/Game/UI/MainMenu/MainMenuLobby.MainMenuLobby_C|GetPlayerBox _lobbymenu) "Hidden")
          (Widget|SetVisibility (Variables|/Game/UI/MainMenu/MainMenuLobby.MainMenuLobby_C|GetButtonBoxA _lobbymenu) "Visible")
          (Variables|/Game/UI/MainMenu/MainMenuLobby.MainMenuLobby_C|SetEnableButtons _lobbymenu true)
          (if (Variables|Default|GetStartPlayList)
            (Default|SelectUI _lobbymenu)))))))

(fn QuitGame
  (Game|QuitGame 0 "Quit"))

(fn ShowMenu
  (params (NewView :type MenuViews%20Enum))
  (bind _output_get (Variables|Default|SetCurrentMenu NewView))
  (switch Utilities|FlowControl|Switch|SwitchonMenuViews _output_get
    (:NewEnumerator0
      (Widget|SetVisibility (Variables|Default|GetlobbyMenu) "Hidden")
      (Widget|SetVisibility (Variables|Default|GetOptionsMenu) "Hidden")
      (Widget|SetVisibility (Variables|Default|GetStreamMenu) "Hidden")
      (Widget|SetVisibility (Variables|Default|GetonlineMenu) "Hidden")
      (Widget|SetVisibility (Variables|Default|GetmainMenu) "Visible")
      (Utilities|String|Reverse (Variables|Default|Getmatinee)))
    (:NewEnumerator1
      (Widget|SetVisibility (Variables|Default|GetmainMenu) "Hidden")
      (Widget|SetVisibility (Variables|Default|GetlobbyMenu) "Visible")
      (Widget|SetVisibility (Variables|Default|GetcustomMenu) "Hidden")
      (Audio|Components|Audio|Play (Variables|Default|Getmatinee)))
    (:NewEnumerator2
      (Widget|SetVisibility (Variables|Default|GetmainMenu) "Hidden")
      (Widget|SetVisibility (Variables|Default|GetOptionsMenu) "Visible"))
    (:NewEnumerator3
      (Widget|SetVisibility (Variables|Default|GetmainMenu) "Hidden")
      (Widget|SetVisibility (Variables|Default|GetStreamMenu) "Visible"))
    (:NewEnumerator4
      (Widget|SetVisibility (Variables|Default|GetlobbyMenu) "Hidden")
      (Widget|SetVisibility (Variables|Default|GetcustomMenu) "Visible"))
    (:NewEnumerator5
      (Widget|SetVisibility (Variables|Default|GetmainMenu) "Hidden")
      (Widget|SetVisibility (Variables|Default|GetonlineMenu) "Visible"))))