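; End-of-match game mode that ranks the four players by wins from PersistentData and presents the results on podiums.
; BeginPlay sorts scores by repeated max extraction, blanking each matched score in a working copy so tied players stay distinct.
; NoSuddenDeath shows the end UI, switches the camera, hides empty podiums and gives ties a shared position.
; Sudden death is unfinished, and its player, pawn and data-actor setup helpers are not run.
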(event EventBeginPlay
  (bind _aspersistent_data (Utilities|Casting|CastToPersistentData (Game|GetGameInstance)))
  (bind _output_get (Variables|Default|SetPersisData _aspersistent_data))
  (Variables|Default|SetGlobalTempScor (Variables|/Game/BluePrints/data/PersistentData.PersistentData_C|GetWins _output_get))
  (for _index (range 0 3)
    ;[1 1 1] set the players in ofder
    (bind _score (CallFunction|GetScoreatRank _index))
    (bind _playernum (CallFunction|GetPlayeratScore _score))
    (Utilities|Array|Insert (Variables|Default|GetPlayerRanking) _playernum _index))
  (CallFunction|NoSuddenDeath))

(fn ConstructionScript)

(fn GetScoreatRank
  (params (Rank :type Integer))
  (bind _output_get (LocalVariables|SetTempoaryScores (Variables|/Game/BluePrints/data/PersistentData.PersistentData_C|GetWins (Variables|Default|GetPersisData))))
  (for _index (range 0 Rank)
    (LocalVariables|SetTempScore (.MaxValue (Math|Integer|MaxOfIntArray _output_get)))
    (Utilities|Array|RemoveIndex (LocalVariables|GetTempoaryScores) (.IndexOfMaxValue (Math|Integer|MaxOfIntArray _output_get))))
  (Utilities|Array|SetArrayElem (Variables|Default|GetScoresSorted) Rank (LocalVariables|GetTempScore) true)
  (return (LocalVariables|GetTempScore)))

(fn GetPlayeratScore
  (params (Score :type Integer))
  (bind _globaltempscor (Variables|Default|GetGlobalTempScor))
  (bind _returnvalue (Utilities|Array|FindItem _globaltempscor Score))
  (bind _output_get (LocalVariables|SetTempValue _returnvalue))
  (Utilities|Array|SetArrayElem _globaltempscor _returnvalue -100)
  (return _output_get))

(fn StartSuddenDeath)

(fn NoSuddenDeath
  (bind _scoressorted (Variables|Default|GetScoresSorted))
  (bind _returnvalue (UserInterface|CreateWidget "/Game/UI/InGame/EndGameUI.EndGameUI_C"))
  (UserInterface|Viewport|AddtoViewport _returnvalue 0)
  (bind _outactors (Actor|GetAllActorsOfClass "/Game/BluePrints/enviroment/PodiumSetUp.PodiumSetUp_C"))
  (Game|Player|SetViewTargetwithBlend (Game|GetPlayerController 0) 0 0.0 "VTBlend_Linear" 0.0 false)
  (for (_array_element _array_index) (Variables|/Game/BluePrints/enviroment/PodiumSetUp.PodiumSetUp_C|GetPodiums (Utilities|Array|Get(acopy) _outactors))
    (if (== (Utilities|Array|Get(acopy) (Variables|/Game/BluePrints/data/PersistentData.PersistentData_C|GetPlayers (Variables|Default|GetPersisData)) (Utilities|Array|Get(acopy) (Variables|Default|GetPlayerRanking) _array_index)) -1)
      ;[1 1 1] no player
      (Rendering|SetActorHiddenInGame _array_element true)
      (Development|PrintString "hide pod" false)
      (elif (== _array_index 0)
        ;[1 1 1] set first player as 1
        (Default|SetUpPodium _array_element)
        (Variables|Default|SetlastPos 0)
        (Variables|Default|SetlastIndex _array_index)
        (Development|PrintString "first player" false)
        (elif (== (Utilities|Array|Get(acopy) _scoressorted _array_index) (Utilities|Array|Get(acopy) _scoressorted (Variables|Default|GetlastIndex)))
          ;[1 1 1] set draw
          (Default|SetUpPodium _array_element (Variables|Default|GetlastPos))
          (Development|PrintString "draw index" false)
          (else
            (bind _result (Math|Integer|IncrementInt (Variables|Default|GetlastPos))
              (:%20%20
                ;[1 1 1] set next
                (Default|SetUpPodium _array_element _result)
                (Variables|Default|SetlastIndex _array_index)
                (Development|PrintString "next player" false)))))))))

(fn SetUpSuddenDeath
  (bind _returnvalue (UserInterface|CreateWidget "/Game/UI/InGame/SuddenDeathGame.SuddenDeathGame_C"))
  (UserInterface|Viewport|AddtoViewport _returnvalue 0))

(fn CheckActorinScene
  (params (Class :type Actor%20Class%20Reference))
  (bind _outactors (Actor|GetAllActorsOfClass Class))
  (return (not (< (Utilities|Array|Length _outactors) 1)) (Utilities|Array|Get(acopy) _outactors)))

(fn SpawnDataActors
  ;[1 1 1] Spawn Data actors here if they are not already in scene, We do not need to cache them all like gamedata
  (bind (_inscene _actor) (CallFunction|CheckActorinScene "/Game/BluePrints/data/GameData.GameData_C"))
  (if _inscene
    (bind _asgame_data (Utilities|Casting|CastToGameData _actor))
    (Variables|Default|SetgameData _asgame_data)
    (else
      (bind _returnvalue (Game|SpawnActorfromClass "/Game/BluePrints/data/GameData.GameData_C" (Math|Transform|MakeTransform "0, 0, 0" "0, 0, 0" "1,1,1") "Undefined" 0 0))
      (Variables|Default|SetgameData _returnvalue)))
  (bind (_inscene_2 _actor_2) (CallFunction|CheckActorinScene "/Game/BluePrints/data/BallData.BallData_C"))
  (if _inscene_2
    (bind _asball_data (Utilities|Casting|CastToBallData _actor_2))
    (Variables|Default|SetBallData _asball_data)
    (else
      (bind _returnvalue_2 (Game|SpawnActorfromClass "/Game/BluePrints/data/BallData.BallData_C" (Math|Transform|MakeTransform "0, 0, 0" "0, 0, 0" "1,1,1") "Undefined" 0 0))
      (Variables|Default|SetBallData _returnvalue_2)))
  (bind _inscene_3 (CallFunction|CheckActorinScene "/Game/BluePrints/data/FractureData.FractureData_C"))
  (if _inscene_3
    _
    (else
      (Game|SpawnActorfromClass "/Game/BluePrints/data/FractureData.FractureData_C" (Math|Transform|MakeTransform "0, 0, 0" "0, 0, 0" "1,1,1") "Undefined" 0 0)))
  (bind _inscene_4 (CallFunction|CheckActorinScene "/Game/BluePrints/data/MutatorData.MutatorData_C"))
  (if (not _inscene_4)
    (Game|SpawnActorfromClass "/Game/BluePrints/data/MutatorData.MutatorData_C" (Math|Transform|MakeTransform "0, 0, 0" "0, 0, 0" "1,1,1") "Undefined" 0 0)))

(fn CreatePlayers
  (bind _persisdata (Variables|Default|GetPersisData))
  (bind _gamedata (Variables|Default|GetgameData))
  (if (Variables|/Game/BluePrints/data/PersistentData.PersistentData_C|GetloadData _persisdata)
    (bind _output_get (Variables|/Game/BluePrints/data/GameData.GameData_C|SetplayerOrder _gamedata (Variables|/Game/BluePrints/data/PersistentData.PersistentData_C|GetPlayers _persisdata)))
    (for _index (range 0 3)
      (bind _asrebound_player_controller (Utilities|Casting|CastToReboundPlayerController (Game|GetPlayerController _index)))
      (if (!= (Utilities|Array|FindItem _output_get _index) -1)
        (Variables|/Game/BluePrints/Core-Gameplay/ReboundPlayerController.ReboundPlayerController_C|SetPlayerID _asrebound_player_controller (Utilities|Array|FindItem _output_get _index))))
    (else
      (for _array_element (Variables|/Game/BluePrints/data/GameData.GameData_C|GetplayerOrder _gamedata)
        (if (!= _array_element -1)
          (bind _returnvalue (Class|GameplayStatics|CreatePlayer _array_element))
          (bind _asrebound_player_controller_2 (Utilities|Casting|CastToReboundPlayerController _returnvalue))
          (if (!= (Pawn|GetControlledPawn _asrebound_player_controller_2) 0)
            (Actor|DestroyActor (Pawn|GetControlledPawn _asrebound_player_controller_2)))
          (bind _output_get_2 (Variables|/Game/BluePrints/Core-Gameplay/ReboundPlayerController.ReboundPlayerController_C|SetPlayerID _asrebound_player_controller_2 _array_element))
          (Development|PrintString (Utilities|String|Append (Utilities|String|ToString(Integer) _output_get_2) "Player created") (Variables|/Game/BluePrints/data/PersistentData.PersistentData_C|GetisDevMode (Variables|Default|GetpersisData))))))))

(fn SpawnPlayerPawns
  (for _array_element (Variables|/Game/BluePrints/data/GameData.GameData_C|GetplayerOrder (Variables|Default|GetgameData))
    (if (!= _array_element -1)
      (bind _asrebound_player_controller (Utilities|Casting|CastToReboundPlayerController (Game|GetPlayerController _array_element)))
      (Default|SpawnPawn _asrebound_player_controller (Transformation|GetActorTransform (Class|GameMode|FindPlayerStart (Game|GetPlayerController _array_element))) (Variables|Default|GetMainPlayerPawn))))
  (bind _outactors (Actor|GetAllActorsOfClass "/Game/BluePrints/Core-Gameplay/Characters/ReboundPlayerCharacter.ReboundPlayerCharacter_C"))
  (bind _output_get (Variables|Default|SetPlayerPawns _outactors))
  (Variables|Default|SetcurrentPlayers (- (Utilities|Array|Length _output_get) 1))
  (Development|PrintString (Utilities|String|BuildString(Integer) "" "No of players " (Utilities|Array|Length _output_get))))