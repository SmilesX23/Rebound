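; Game mode for Rebound's local multiplayer dodgeball matches, running rounds from player creation and pawn spawning to scoring and match end.
; Bound round-phase events drive spawning, UI and layered battle music intensity.
; Deaths score as Score Per Kill or Last Man Alive, ending rounds as players run out.
; Wins persist in the PersistentData game instance, which advances the level playlist to EndLevel, or SuddenDeath on ties.
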(event Custom|PostRoundCall
  (Math|Integer|IncrementInt (Variables|Default|Getround)
    (:%20%20
      (CallFunction|CheckWinConditions)
      (CallFunction|DespawnPlayerPawns))))

(event Custom|PreRoundCall
  (CallFunction|SpawnPlayerPawns))

(event Custom|LoadLevel
  (params (Name :type Name))
  (Utilities|FlowControl|Delay 5.0)
  ;[1 1 1] load level
  (Game|OpenLevel(byName) Name))

(event Custom|PlayerDiedMusicUpdate
  (bind _battlemusic (Variables|Default|GetBattleMusic))
  (if (<= (Variables|Default|GetcurrentPlayers) 2)
    (Audio|Parameter|SetFloatParameter _battlemusic "LowLayer" 1.0 :!class /Script/Engine.AudioComponent)
    (if (<= (Variables|Default|GetcurrentPlayers) 1)
      (Audio|Parameter|SetFloatParameter _battlemusic "MediumLayer" 1.0 :!class /Script/Engine.AudioComponent))))

(event Custom|StartGameCall
  (bind _gamedata (Variables|Default|GetgameData))
  (bind _aspersistent_data (Utilities|Casting|CastToPersistentData (Game|GetGameInstance)))
  (if (Variables|/Game/BluePrints/data/PersistentData.PersistentData_C|GetloadData _aspersistent_data)
    (Variables|/Game/BluePrints/data/GameData.GameData_C|SetplayerOrder _gamedata (Variables|/Game/BluePrints/data/PersistentData.PersistentData_C|GetPlayers _aspersistent_data)))
  (CallFunction|CreatePlayers (Variables|/Game/BluePrints/data/GameData.GameData_C|GetplayerOrder _gamedata)))

(event Custom|StartRoundCall
  (bind _battlemusic (Variables|Default|GetBattleMusic))
  (Variables|Default|SetLastManAliveErrorCheck -1)
  (Audio|Parameter|SetFloatParameter _battlemusic "MediumLayer" 0.0 :!class /Script/Engine.AudioComponent)
  (Audio|Parameter|SetFloatParameter _battlemusic "HighLayer" 0.0 :!class /Script/Engine.AudioComponent))

(event Custom|EndRoundCall
  (Widget|SetVisibility (Variables|Default|GetEndRoundUI) "Visible"))

(event EventBeginPlay
  (bind _scores (Variables|Default|GetScores))
  (bind _battlemusic (Variables|Default|GetBattleMusic))
  (Audio|Components|Audio|Play _battlemusic 0.0)
  (Audio|Parameter|SetFloatParameter _battlemusic "MediumLayer" 0.0 :!class /Script/Engine.AudioComponent)
  (Audio|Parameter|SetFloatParameter _battlemusic "HighLayer" 0.0 :!class /Script/Engine.AudioComponent)
  (CallFunction|SpawnDataActors)
  (EventDispatchers|BindEventtoStartGame (delegate Custom|StartGameCall))
  (EventDispatchers|BindEventtoStartRound (delegate Custom|StartRoundCall))
  (EventDispatchers|BindEventtoEndRound (delegate Custom|EndRoundCall))
  (EventDispatchers|BindEventtoPostRound (delegate Custom|PostRoundCall))
  (EventDispatchers|BindEventtoPreRound (delegate Custom|PreRoundCall))
  (EventDispatchers|BindEventtoPlayerHasDied (delegate Custom|PlayerDiedMusicUpdate))
  (bind _returnvalue (UserInterface|CreateWidget "/Game/UI/InGame/InGameUI.InGameUI_C"))
  (bind _returnvalue_2 (UserInterface|CreateWidget "/Game/UI/InGame/EndRound.EndRound_C"))
  (bind _returnvalue_3 (UserInterface|CreateWidget "/Game/UI/InGame/StartGame.StartGame_C"))
  (bind _output_get (Variables|Default|SetEndRoundUI _returnvalue_2))
  (UserInterface|Viewport|AddtoViewport _returnvalue 0)
  (Widget|SetVisibility _output_get "Hidden")
  (bind _aspersistent_data (Utilities|Casting|CastToPersistentData (Game|GetGameInstance)))
  (bind _output_get_2 (Variables|Default|SetPersisData _aspersistent_data))
  (for (_ _array_index) _scores
    (Utilities|Array|SetArrayElem _scores _array_index (Utilities|Array|Get(acopy) (Variables|/Game/BluePrints/data/PersistentData.PersistentData_C|GetWins _output_get_2) _array_index)))
  (bind _output_get_3 (Variables|Default|SetMaxRounds (Utilities|Array|Get(acopy) (Variables|/Game/BluePrints/data/PersistentData.PersistentData_C|Getrounds _aspersistent_data) (Variables|/Game/BluePrints/data/PersistentData.PersistentData_C|GetplaylistID _aspersistent_data))))
  (if (== _output_get_3 0)
    (Variables|Default|SetMaxRounds 5)))

(event EventTick
  (params (DeltaSeconds :type Float%20%28single-precision%29))
  (if (not (Variables|Default|GetHasStarted))
    (Default|CallStartGame)
    (Default|CallPreRound)
    (Variables|Default|SetHasStarted true)))

(fn ConstructionScript)

(fn CreatePlayers
  (params (PlayerIndexArray :type Array%20of%20Integers))
  (bind _aspersistent_data (Utilities|Casting|CastToPersistentData (Game|GetGameInstance)))
  (if (Variables|/Game/BluePrints/data/PersistentData.PersistentData_C|GetloadData _aspersistent_data)
    (for _index (range 0 3)
      (bind _asrebound_player_controller (Utilities|Casting|CastToReboundPlayerController (Game|GetPlayerController _index)))
      (if (!= (Utilities|Array|FindItem PlayerIndexArray _index) -1)
        (Variables|/Game/BluePrints/Core-Gameplay/ReboundPlayerController.ReboundPlayerController_C|SetPlayerID _asrebound_player_controller (Utilities|Array|FindItem PlayerIndexArray _index))))
    (else
      (for _array_element PlayerIndexArray
        (if (!= _array_element -1)
          (bind _returnvalue (Class|GameplayStatics|CreatePlayer _array_element))
          (bind _asrebound_player_controller_2 (Utilities|Casting|CastToReboundPlayerController _returnvalue))
          (if (!= (Pawn|GetControlledPawn _asrebound_player_controller_2) 0)
            (Actor|DestroyActor (Pawn|GetControlledPawn _asrebound_player_controller_2)))
          (bind _output_get (Variables|/Game/BluePrints/Core-Gameplay/ReboundPlayerController.ReboundPlayerController_C|SetPlayerID _asrebound_player_controller_2 _array_element))
          (Development|PrintString (Utilities|String|Append (Utilities|String|ToString(Integer) _output_get) "Player created") (Variables|/Game/BluePrints/data/PersistentData.PersistentData_C|GetisDevMode (Variables|Default|GetpersisData))))))))

(fn SpawnPlayerPawns
  (for _array_element (Variables|/Game/BluePrints/data/GameData.GameData_C|GetplayerOrder (Variables|Default|GetgameData))
    (if (!= _array_element -1)
      (bind _asrebound_player_controller (Utilities|Casting|CastToReboundPlayerController (Game|GetPlayerController _array_element)))
      (Default|SpawnPawn _asrebound_player_controller (Transformation|GetActorTransform (Class|GameMode|FindPlayerStart (Game|GetPlayerController _array_element))) (Variables|Default|GetMainPlayerPawn))))
  (bind _outactors (Actor|GetAllActorsOfClass "/Game/BluePrints/Core-Gameplay/Characters/ReboundPlayerCharacter.ReboundPlayerCharacter_C"))
  (bind _output_get (Variables|Default|SetPlayerPawns _outactors))
  (Variables|Default|SetcurrentPlayers (- (Utilities|Array|Length _output_get) 1)))

(fn PlayerDied
  (params (BallID :type Integer) (HitID :type Integer) (KilledByDodgeball :type Boolean) (player :type Rebound%20Player%20Character%20Object%20Reference))
  (bind _returnvalue (Transformation|GetActorLocation player))
  (bind _scores (Variables|Default|GetScores))
  (bind _scores_2 (Variables|Default|GetScores))
  (bind _item (Utilities|Array|Get(acopy) _scores BallID))
  (if (not (Game|IsActorBeingDestroyed player))
    (Utilities|Array|RemoveItem (Variables|Default|GetPlayerPawns) player)
    (Default|DropBall player false)
    (Effects|SpawnEmitteratLocation "/Game/Art/Particles/Explosion.Explosion" _returnvalue)
    (bind _returnvalue_2 (Game|SpawnActorfromClass "/Game/BluePrints/Core-Gameplay/Characters/DeathWaveEffect.DeathWaveEffect_C" (Math|Transform|MakeTransform _returnvalue "0, 0, 0" "1,1,1.000000") "Undefined" 0 0))
    (Rendering|Material|SetVectorParameterValueonMaterials (Variables|/Game/BluePrints/Core-Gameplay/Characters/DeathWaveEffect.DeathWaveEffect_C|GetDestructible _returnvalue_2) "WireColour" (Math|Conversions|ToVector(LinearColor) (.charcolour (Utilities|Array|Get(acopy) (Variables|/Game/BluePrints/data/PersistentData.PersistentData_C|GetPlayerCharacters (Variables|Default|GetPersisData)) (Variables|/Game/BluePrints/Core-Gameplay/ReboundPlayerController.ReboundPlayerController_C|GetPlayerID (Default|GetReboundPlayerController player))))))
    (Actor|DestroyActor player)
    (Default|CallPlayerHasDied)
    (switch Utilities|FlowControl|Switch|SwitchonScoreType (Variables|Default|GetScoreType)
      (:NewEnumerator0
        ;[1 1 1] ScorePerKill
        (if KilledByDodgeball
          (if (== BallID HitID)
            (Utilities|Array|SetArrayElem _scores BallID (- _item 1))
            (else
              (Utilities|Array|SetArrayElem _scores BallID (+ _item 1)))))
        (bind _result (Math|Integer|DecrementInt (Variables|Default|GetcurrentPlayers))
          (:%20%20
            (if (<= _result 0)
              (Default|CallEndRound)))))
      (:NewEnumerator1
        ;[1 1 1] Last Man Standing
        (bind _result_2 (Math|Integer|DecrementInt (Variables|Default|GetcurrentPlayers))
          (:%20%20
            (if (<= _result_2 0)
              (bind _outactors (Actor|GetAllActorsOfClass "/Game/BluePrints/Core-Gameplay/Characters/ReboundPlayerCharacter.ReboundPlayerCharacter_C"))
              (if (not (== (Utilities|Array|Length _outactors) 0))
                (Utilities|Array|SetArrayElem _scores_2 (Variables|/Game/BluePrints/Core-Gameplay/ReboundPlayerController.ReboundPlayerController_C|GetPlayerID (Default|GetReboundPlayerController (Utilities|Array|Get(acopy) _outactors))) (+ (Utilities|Array|Get(acopy) _scores_2 (Variables|/Game/BluePrints/Core-Gameplay/ReboundPlayerController.ReboundPlayerController_C|GetPlayerID (Default|GetReboundPlayerController (Utilities|Array|Get(acopy) _outactors)))) 1))
                (Variables|Default|SetLastManAliveErrorCheck (Variables|/Game/BluePrints/Core-Gameplay/ReboundPlayerController.ReboundPlayerController_C|GetPlayerID (Default|GetReboundPlayerController (Utilities|Array|Get(acopy) _outactors))))
                (else
                  (CallFunction|LastManAliveCheck)))
              (Default|CallEndRound))))))))

(fn FindPlayerStart
  (params (Player :type Controller%20Object%20Reference) (IncomingName :type String))
  (bind _asrebound_player_controller (Utilities|Casting|CastToReboundPlayerController Player)
    (:then
      (bind _outactors (Actor|GetAllActorsOfClass "/Script/Engine.PlayerStart"))
      (return (Utilities|Array|Get(acopy) _outactors (Variables|/Game/BluePrints/Core-Gameplay/ReboundPlayerController.ReboundPlayerController_C|GetPlayerID _asrebound_player_controller))))
    (:CastFailed
      (bind _outactors_2 (Actor|GetAllActorsOfClass "/Script/Engine.PlayerStart"))
      (return (Utilities|Array|Get(acopy) _outactors_2)))))

(fn SpawnDataActors
  ;[1 1 1] Spawn Data actors here if they are not already in scene, We do not need to cache them all like gamedata
  (bind (_inscene _actor) (CallFunction|CheckActorinScene "/Game/BluePrints/data/GameData.GameData_C"))
  (if _inscene
    (bind _asgame_data (Utilities|Casting|CastToGameData _actor))
    (Variables|Default|SetgameData _asgame_data)
    (else
      (bind _returnvalue (Game|SpawnActorfromClass "/Game/BluePrints/data/GameData.GameData_C" (Math|Transform|MakeTransform "0, 0, 0" "0, 0, 0" "1,1,1") "Undefined" 0 0))
      (Variables|Default|SetgameData _returnvalue)))
  (bind _inscene_2 (CallFunction|CheckActorinScene "/Game/BluePrints/data/BallData.BallData_C"))
  (if _inscene_2
    _
    (else
      (Game|SpawnActorfromClass "/Game/BluePrints/data/BallData.BallData_C" (Math|Transform|MakeTransform "0, 0, 0" "0, 0, 0" "1,1,1") "Undefined" 0 0)))
  (bind _inscene_3 (CallFunction|CheckActorinScene "/Game/BluePrints/data/FractureData.FractureData_C"))
  (if _inscene_3
    _
    (else
      (Game|SpawnActorfromClass "/Game/BluePrints/data/FractureData.FractureData_C" (Math|Transform|MakeTransform "0, 0, 0" "0, 0, 0" "1,1,1") "Undefined" 0 0)))
  (bind _inscene_4 (CallFunction|CheckActorinScene "/Game/BluePrints/data/MutatorData.MutatorData_C"))
  (if (not _inscene_4)
    (Game|SpawnActorfromClass "/Game/BluePrints/data/MutatorData.MutatorData_C" (Math|Transform|MakeTransform "0, 0, 0" "0, 0, 0" "1,1,1") "Undefined" 0 0)))

(fn CheckActorinScene
  (params (Class :type Actor%20Class%20Reference))
  (bind _outactors (Actor|GetAllActorsOfClass Class))
  (return (not (< (Utilities|Array|Length _outactors) 1)) (Utilities|Array|Get(acopy) _outactors)))

(fn CheckWinConditions
  (bind _scores (Variables|Default|GetScores))
  (bind (_indexofmaxvalue _maxvalue) (Math|Integer|MaxOfIntArray _scores))
  (if (>= (Variables|Default|Getround) (Variables|Default|GetMaxRounds))
    (for (_array_element _array_index) (Variables|Default|GetScores)
      (if (> _array_element (LocalVariables|GetWinningScore))
        (LocalVariables|SetWinningPlayer _array_index)
        (LocalVariables|SetWinningScore _array_element)))
    (Development|PrintString (Utilities|String|Append "Player " (Utilities|String|ToString(Integer) (LocalVariables|GetWinningPlayer)) " wins") (Variables|/Game/BluePrints/data/PersistentData.PersistentData_C|GetisDevMode (Variables|Default|GetpersisData)) true "(R=1.000000,G=0.552805,B=0.113152,A=1.000000)" 5.0 :!label _label)
    (Default|CallEndGame)
    (CallFunction|AdvancePlaylist)
    (else
      (switch Utilities|FlowControl|Switch|SwitchonScoreType (Variables|Default|GetScoreType)
        (:NewEnumerator0
          (if (>= _maxvalue (Variables|Default|GetPointsToWin))
            (LocalVariables|SetWinningPlayer _indexofmaxvalue)
            (goto _label)))))))

(fn DespawnPlayerPawns
  (bind _playerpawns (Variables|Default|GetPlayerPawns))
  (for _array_element _playerpawns
    (Actor|DestroyActor _array_element))
  (Utilities|Array|Clear _playerpawns))

(fn AdvancePlaylist
  (bind _persisdata (Variables|Default|GetPersisData))
  (bind _wins (Variables|/Game/BluePrints/data/PersistentData.PersistentData_C|GetWins _persisdata))
  (bind _aspersistent_data (Utilities|Casting|CastToPersistentData (Game|GetGameInstance)))
  ;[1 1 1] set overall Scores
  (for (_array_element _array_index) (Variables|Default|GetScores)
    (Utilities|Array|SetArrayElem (Variables|/Game/BluePrints/data/PersistentData.PersistentData_C|GetWins _aspersistent_data) _array_index _array_element true))
  (if (Variables|/Game/BluePrints/data/PersistentData.PersistentData_C|GetloadData _aspersistent_data)
    (bind _result (Math|Integer|IncrementInt (Variables|/Game/BluePrints/data/PersistentData.PersistentData_C|GetplaylistID _aspersistent_data))
      (:%20%20
        (if (== _result (Utilities|Array|Length (Variables|/Game/BluePrints/data/PersistentData.PersistentData_C|GetLevelList _aspersistent_data)))
          ;[1 1 1] loading screen vid
          (bind _returnvalue (UserInterface|CreateWidget "/Game/UI/loadingScreen/InfoLoadingScreen.InfoLoadingScreen_C"))
          (UserInterface|Viewport|AddtoViewport _returnvalue 0)
          (for _array_element_2 _wins
            (if (== (.MaxValue (Math|Integer|MaxOfIntArray _wins)) _array_element_2)
              (Math|Integer|IncrementInt (LocalVariables|GetNoOfWinners))))
          (if (not (>= (LocalVariables|GetNoOfWinners) 2))
            (CallFunction|LoadLevel "EndLevel")
            (else
              (CallFunction|LoadLevel "SuddenDeath")))
          (else
            ;[1 1 1] loading screen vid
            (bind _returnvalue_2 (UserInterface|CreateWidget "/Game/UI/loadingScreen/InfoLoadingScreen.InfoLoadingScreen_C"))
            (UserInterface|Viewport|AddtoViewport _returnvalue_2 0)
            (CallFunction|LoadLevel (Utilities|Array|Get(acopy) (Variables|/Game/BluePrints/data/PersistentData.PersistentData_C|GetLevelList _aspersistent_data) _result))))))
    (else
      ;[1 1 1] loading screen vid
      (bind _returnvalue_3 (UserInterface|CreateWidget "/Game/UI/loadingScreen/InfoLoadingScreen.InfoLoadingScreen_C"))
      (UserInterface|Viewport|AddtoViewport _returnvalue_3 0)
      ;[1 1 1] load level
      (Game|OpenLevel(byName) "MainMenu"))))

(fn LastManAliveCheck
  (bind _lastmanaliveerrorcheck (Variables|Default|GetLastManAliveErrorCheck))
  (bind _scores (Variables|Default|GetScores))
  (if (!= _lastmanaliveerrorcheck -1)
    (Utilities|Array|SetArrayElem _scores _lastmanaliveerrorcheck (- (Utilities|Array|Get(acopy) _scores _lastmanaliveerrorcheck) 1))
    (else
      (Development|PrintString "NoLastManAliveError" (Variables|/Game/BluePrints/data/PersistentData.PersistentData_C|GetisDevMode (Variables|Default|GetpersisData))))))