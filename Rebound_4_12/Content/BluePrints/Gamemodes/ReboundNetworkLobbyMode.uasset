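; Game mode for the Rebound network lobby, announcing player joins with a debug print and handling the start of play.
; On authority, PlayGame flags PersistentData in the game instance to load data, enables seamless travel, and hides the UI on every NetworkLobbyController.
; The servertravel command to the TheRing network test level and the CallMoveServer call are disconnected, so no travel happens here.
; A helper returns a player's start transform.
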(event Custom|PlayGame
  (Networking|SwitchHasAuthority
    (:Authority
      (bind _aspersistent_data (Utilities|Casting|CastToPersistentData (Game|GetGameInstance)))
      (Variables|/Game/BluePrints/data/PersistentData.PersistentData_C|SetloadData _aspersistent_data true)
      (Variables|Default|SetbUseSeamlessTravel true)
      (bind _outactors (Actor|GetAllActorsOfClass "/Game/BluePrints/Core-Gameplay/NetworkLobbyController.NetworkLobbyController_C"))
      (for _array_element _outactors
        (Default|HideUI _array_element)))))

(event EventBeginPlay)

(event EventPostLogin
  (params (NewPlayer :type Player%20Controller%20Object%20Reference))
  (Development|PrintString "player joined" true true "(R=0.224048,G=1.000000,B=0.000000,A=1.000000)" 5.0))

(fn ConstructionScript)

(fn GetPlayerStart
  (params (player :type Player%20Controller%20Object%20Reference))
  (return (Transformation|GetActorTransform (Class|GameMode|FindPlayerStart player))))