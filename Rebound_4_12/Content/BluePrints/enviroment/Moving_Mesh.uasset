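; Environment actor that moves itself along a looping path of transforms stored in WallTrans.
; Every tick, MoveMesh lerps the full actor transform from the current waypoint to the next, using elapsed time times Speed over segment distance, so travel speed stays constant.
; At the end of a segment, TogglePos advances the index, wrapping to the first, then recomputes the distance and restarts the timer.
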(event EventBeginPlay
  (bind _walltrans (Variables|Default|GetWallTrans))
  (Variables|Default|Setdistance (Math|Vector|VectorLength (- (.location (Utilities|Array|Get(acopy) _walltrans)) (.location (Utilities|Array|Get(acopy) _walltrans 1)))))
  (Variables|Default|SetstartTime (Utilities|Time|GetGameTimeinSeconds)))

(event EventTick
  (params (DeltaSeconds :type Float%20%28single-precision%29))
  (CallFunction|MoveMesh))

(fn ConstructionScript)

(fn MoveMesh
  (bind _returnvalue (Utilities|Time|GetGameTimeinSeconds))
  (bind _walltrans (Variables|Default|GetWallTrans))
  (bind _starttime (Variables|Default|GetstartTime))
  (bind _distance (Variables|Default|Getdistance))
  (bind _wallindex (Variables|Default|GetWallIndex))
  (bind _speed (Variables|Default|GetSpeed))
  (bind _returnvalue_2 (- _returnvalue _starttime))
  (bind _returnvalue_3 (+ _wallindex 1))
  (bind _returnvalue_4 (* _returnvalue_2 _speed))
  (bind _returnvalue_5 (/ _returnvalue_4 _distance))
  (Transformation|SetActorTransform (Math|Transform|Lerp(Transform) (Utilities|Array|Get(acopy) _walltrans _wallindex) (Utilities|Array|Get(acopy) _walltrans (select (== _returnvalue_3 (Utilities|Array|Length (Variables|Default|GetWallTrans))) 0 _returnvalue_3)) _returnvalue_5))
  (if (>= _returnvalue_5 1.0)
    (CallFunction|TogglePos)))

(fn TogglePos
  (bind _walltrans (Variables|Default|GetWallTrans))
  (if (< (Variables|Default|GetWallIndex) (- (Utilities|Array|Length (Variables|Default|GetWallTrans)) 1))
    (Math|Integer|IncrementInt (Variables|Default|GetWallIndex)
      (:%20%20
        _))
    (else
      (Variables|Default|SetWallIndex 0)))
  (Variables|Default|Setdistance (Math|Vector|VectorLength (- (.location (Utilities|Array|Get(acopy) _walltrans (Variables|Default|GetWallIndex))) (.location (Utilities|Array|Get(acopy) _walltrans (select (== (+ (Variables|Default|GetWallIndex) 1) (Utilities|Array|Length (Variables|Default|GetWallTrans))) 0 (+ (Variables|Default|GetWallIndex) 1)))))))
  (Variables|Default|SetstartTime (Utilities|Time|GetGameTimeinSeconds)))