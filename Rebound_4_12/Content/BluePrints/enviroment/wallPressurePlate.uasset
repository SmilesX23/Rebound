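; Pressure plate that toggles a wall when ReboundPlayerCharacter actors step on or off it.
; A box trigger checks its overlap count, so only the first player entering and the last one leaving change its state.
; Each change recolors the mesh through material vector parameters, yellow when occupied and green when vacated, then calls ToggleWall to signal the flip.
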(event OnComponentBeginOverlap(Box)
  (params (OtherActor :type Actor%20Object%20Reference) (OtherComp :type Primitive%20Component%20Object%20Reference) (OtherBodyIndex :type Integer) (bFromSweep :type Boolean) (SweepResult :type Hit%20Result%20Structure%20%28by%20ref%29))
  (bind _static_mesh (Variables|Default|Getstatic%20mesh))
  (Utilities|Casting|CastToReboundPlayerCharacter OtherActor)
  (if (== (Utilities|Array|Length (Collision|GetOverlappingActors (Variables|Default|GetBox) "/Game/BluePrints/Core-Gameplay/Characters/ReboundPlayerCharacter.ReboundPlayerCharacter_C" :!class /Script/Engine.PrimitiveComponent)) 1)
    (Rendering|Material|SetVectorParameterValueonMaterials _static_mesh "Albedo_Tint" (Math|Conversions|ToVector(LinearColor) "(R=0.054902,G=0.051952,B=0.028219,A=1.000000)"))
    (Rendering|Material|SetVectorParameterValueonMaterials _static_mesh "Emissive_Color" (Math|Conversions|ToVector(LinearColor) "(R=1.000000,G=0.929063,B=0.000000,A=1.000000)"))
    (Default|CallToggleWall)))

(event OnComponentEndOverlap(Box)
  (params (OtherActor :type Actor%20Object%20Reference) (OtherComp :type Primitive%20Component%20Object%20Reference) (OtherBodyIndex :type Integer))
  (bind _static_mesh (Variables|Default|Getstatic%20mesh))
  (Utilities|Casting|CastToReboundPlayerCharacter OtherActor)
  (if (== (Utilities|Array|Length (Collision|GetOverlappingActors (Variables|Default|GetBox) "/Game/BluePrints/Core-Gameplay/Characters/ReboundPlayerCharacter.ReboundPlayerCharacter_C" :!class /Script/Engine.PrimitiveComponent)) 0)
    (Rendering|Material|SetVectorParameterValueonMaterials _static_mesh "Albedo_Tint" (Math|Conversions|ToVector(LinearColor) "(R=0.035294,G=0.054902,B=0.031373,A=1.000000)"))
    (Rendering|Material|SetVectorParameterValueonMaterials _static_mesh "Emissive_Color" (Math|Conversions|ToVector(LinearColor) "(R=0.000000,G=1.000000,B=0.000000,A=1.000000)"))
    (Default|CallToggleWall)))

(fn ConstructionScript)