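; WallBP is a wall actor that is either static or breakable, shattering and fading away when fractured.
; StatsAssigned uses FractureStats to show the static mesh, or hide it and load a fracture mesh into the Destructible.
; On fracture, heavy radius damage and an impulse scatter it with an explosion, wireframe materials and pawn/world-static collision ignored.
; Tick then lowers the Alpha material parameter via ChangeBrightness until the actor destroys itself.
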(event OnComponentFracture(Destructible)
  (params (HitPoint :type Vector%20%28by%20ref%29 :default "0, 0, 0") (HitDirection :type Vector%20%28by%20ref%29 :default "0, 0, 0"))
  (bind _destructible (Variables|Default|GetDestructible))
  (bind _destructible_2 (Variables|Default|GetDestructible))
  (bind _destructible_3 (Variables|Default|GetDestructible))
  (Development|PrintString "on fracture")
  (Class|DestructibleComponent|ApplyRadiusDamage _destructible_2 4e+03 (Transformation|GetWorldLocation _destructible_2) 2e+03 2e+03 true)
  (Variables|Default|SetisFractured true)
  (Effects|SpawnEmitteratLocation "/Game/Art/Particles/Explosion.Explosion" (Transformation|GetActorLocation))
  (Physics|AddRadialImpulse _destructible_3 (Transformation|GetWorldLocation _destructible_3) 5e+01 1e+02 "RIF_Constant" false)
  (Rendering|Material|CreateDynamicMaterialInstance _destructible_3 0 "/Game/Art/Test/Wireframe_Inst.Wireframe_Inst" :!class /Script/Engine.PrimitiveComponent)
  (Rendering|Material|CreateDynamicMaterialInstance _destructible_3 1 "/Game/Art/Test/Wireframe_Inst.Wireframe_Inst" :!class /Script/Engine.PrimitiveComponent)
  (Collision|SetCollisionResponsetoChannel _destructible "ECC_WorldStatic" "ECR_Ignore")
  (Collision|SetCollisionResponsetoChannel _destructible "ECC_Pawn" "ECR_Ignore"))

(event EventBeginPlay
  (bind _aspersistent_data (Utilities|Casting|CastToPersistentData (Game|GetGameInstance)))
  (Variables|Default|SetpersisData _aspersistent_data))

(event EventTick
  (params (DeltaSeconds :type Float%20%28single-precision%29))
  (if (Variables|Default|GetisFractured)
    (CallFunction|ChangeBrightness DeltaSeconds)))

(fn ConstructionScript)

(fn GetDestructable
  (return (Variables|Default|GetDestructible)))

(fn ChangeBrightness
  (params (DeltaTime :type Float%20%28single-precision%29))
  (bind _output_get (Variables|Default|SetBrightness (- (Variables|Default|GetBrightness) (* DeltaTime (Variables|Default|GetdecaySpeed)))))
  (Rendering|Material|SetScalarParameterValueonMaterials (Variables|Default|GetDestructible) "Alpha" _output_get)
  (if (<= (+ _output_get 0.1) 0.0)
    (Actor|DestroyActor)))

(fn StatsAssigned
  (bind _static (Variables|Default|GetStatic))
  (if (.fracture (Variables|Default|GetFractureStats))
    (Rendering|SetVisibility _static false false)
    (Collision|SetCollisionEnabled _static "NoCollision")
    (Class|DestructibleComponent|SetDestructibleMesh (Variables|Default|GetDestructible) (.fracmesh (Variables|Default|GetFractureStats)))
    (else
      (Rendering|SetVisibility _static true false)
      (Collision|SetCollisionEnabled _static "QueryAndPhysics"))))