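; PodiumSetUp builds the end-of-level podium display from the ranking and scores in EndLevelMode.
; SetPodiums spawns each ranked player's skeletal mesh at its podium position, looping an idle animation with a dynamic material tinted to the player's colour.
; It writes position and score into matching text actors in that colour, with tied neighbours sharing a place number.
; The event graph's camera view switch is unconnected.
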(event EventBeginPlay)

(event EventActorBeginOverlap
  (params (OtherActor :type Actor%20Object%20Reference)))

(event EventTick
  (params (DeltaSeconds :type Float%20%28single-precision%29)))

(fn ConstructionScript)

(fn SetPodiums
  (bind _placesat (LocalVariables|GetPlacesat))
  (bind _asend_level_mode (Utilities|Casting|CastToEndLevelMode (Game|GetGameMode)))
  (for (_array_element _array_index) (Variables|/Game/BluePrints/Gamemodes/EndLevelMode.EndLevelMode_C|GetPlayerRanking _asend_level_mode)
    ;[1 1 1] Set Mesh
    (bind _returnvalue (Game|SpawnActorfromClass "/Script/Engine.SkeletalMeshActor" (Transformation|GetActorTransform (Utilities|Array|Get(acopy) (Variables|Default|GetPodiumPositions) _array_index)) "Undefined" 0 0))
    (Class|SkinnedMeshComponent|SetSkeletalMesh (Variables|/Script/Engine.SkeletalMeshActor|GetSkeletalMeshComponent _returnvalue) (.mesh (Utilities|Array|Get(acopy) (Variables|/Game/BluePrints/data/PersistentData.PersistentData_C|GetPlayerCharacters (Variables|/Game/BluePrints/Gamemodes/EndLevelMode.EndLevelMode_C|GetPersisData _asend_level_mode)) _array_element)) true)
    (Components|Animation|PlayAnimation (Variables|/Script/Engine.SkeletalMeshActor|GetSkeletalMeshComponent _returnvalue) "/Game/Art/Character/Animations/Idle_001.Idle_001" true)
    (bind _returnvalue_2 (Rendering|Material|CreateDynamicMaterialInstance (Variables|/Script/Engine.SkeletalMeshActor|GetSkeletalMeshComponent _returnvalue) 0 "/Game/Art/Character/Character_new/playerColourInstance.playerColourInstance" :!class /Script/Engine.PrimitiveComponent))
    (Rendering|Material|SetVectorParameterValue _returnvalue_2 "playerColour" (.charcolour (Utilities|Array|Get(acopy) (Variables|/Game/BluePrints/data/PersistentData.PersistentData_C|GetPlayerCharacters (Variables|/Game/BluePrints/Gamemodes/EndLevelMode.EndLevelMode_C|GetPersisData _asend_level_mode)) _array_element)) :!class /Script/Engine.MaterialInstanceDynamic)
    ;[1 1 1] Set Text and Colour
    (Utilities|IsValid (Utilities|Array|Get(acopy) (Variables|Default|GetScoresText) (- _array_index 1))
      (:Is%20Valid
        (if (== (Utilities|Array|Get(acopy) (Variables|/Game/BluePrints/Gamemodes/EndLevelMode.EndLevelMode_C|GetScoresSorted _asend_level_mode) (- _array_index 1)) (Utilities|Array|Get(acopy) (Variables|/Game/BluePrints/Gamemodes/EndLevelMode.EndLevelMode_C|GetScoresSorted _asend_level_mode) _array_index))
          (Rendering|Components|TextRender|SetText (Variables|/Script/Engine.TextRenderActor|GetTextRender (Utilities|Array|Get(acopy) (Variables|Default|GetScoresText) _array_index)) (Utilities|Text|ToText(String) (Utilities|String|Append "Pos: " (Utilities|String|ToString(Integer) _placesat) " 
Score:" (Utilities|String|ToString(Integer) (Utilities|Array|Get(acopy) (Variables|/Game/BluePrints/Gamemodes/EndLevelMode.EndLevelMode_C|GetScoresSorted _asend_level_mode) _array_index)))))
          (else
            (Math|Integer|IncrementInt _placesat :!label _label
              (:%20%20
                (Rendering|Components|TextRender|SetText (Variables|/Script/Engine.TextRenderActor|GetTextRender (Utilities|Array|Get(acopy) (Variables|Default|GetScoresText) _array_index)) (Utilities|Text|ToText(String) (Utilities|String|Append "Pos: " (Utilities|String|ToString(Integer) _placesat) " 
Score: " (Utilities|String|ToString(Integer) (Utilities|Array|Get(acopy) (Variables|/Game/BluePrints/Gamemodes/EndLevelMode.EndLevelMode_C|GetScoresSorted _asend_level_mode) _array_index))))))))))
      (:Is%20Not%20Valid
        (goto _label)))
    (Rendering|Components|TextRender|SetTextRenderColor (Variables|/Script/Engine.TextRenderActor|GetTextRender (Utilities|Array|Get(acopy) (Variables|Default|GetScoresText) _array_index)) (Math|Conversions|ToColor(LinearColor) (.charcolour (Utilities|Array|Get(acopy) (Variables|/Game/BluePrints/data/PersistentData.PersistentData_C|GetPlayerCharacters (Variables|/Game/BluePrints/Gamemodes/EndLevelMode.EndLevelMode_C|GetPersisData _asend_level_mode)) _array_element)))))
  (Development|PrintString "Complete"))