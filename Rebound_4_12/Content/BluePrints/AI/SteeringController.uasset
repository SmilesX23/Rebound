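; SteeringController is an unfinished AI helper that picks a dodgeball target for the second player's ReboundPlayerCharacter, cached after a one-second delay.
; Each Tick keeps a valid, uncarried target and draws a red debug line to it, otherwise rescanning all DodgeBalls.
; The scan seeks the uncarried ball nearest the controller itself, not the character, and never resets its stored best distance.
; Movement calls exist but are unconnected, so nothing steers yet.
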(event EventTick
  (params (DeltaSeconds :type Float%20%28single-precision%29))
  (Utilities|FlowControl|Sequence
    (:then_0
      (if (== (Variables|Default|GettargetBall) 0)
        (CallFunction|SetCurrentBall :!label _label)
        (elif (CallFunction|CheckBall)
          (Rendering|Debug|DrawDebugLine (Transformation|GetActorLocation (Variables|Default|GetCharacter)) (Transformation|GetActorLocation (Variables|Default|GettargetBall)) "(R=1.000000,G=0.000000,B=0.039438,A=1.000000)" 0.0 5.0)
          (else
            (goto _label)))))))

(event EventBeginPlay
  (Utilities|FlowControl|Delay 1.0)
  (bind _asrebound_player_character (Utilities|Casting|CastToReboundPlayerCharacter (Pawn|GetControlledPawn (Game|GetPlayerController 1))))
  (Variables|Default|SetCharacter _asrebound_player_character))

(fn ConstructionScript)

(fn SetCurrentBall
  (bind _outactors (Actor|GetAllActorsOfClass "/Game/BluePrints/Core-Gameplay/Dodgeballs/DodgeBall.DodgeBall_C"))
  (for (_array_element _array_index) _outactors
    (if (and (not (Variables|/Game/BluePrints/Core-Gameplay/Dodgeballs/DodgeBall.DodgeBall_C|GetIsCarried _array_element)) (< (Transformation|GetDistanceTo _array_element self) (LocalVariables|GetlowDis)))
      (LocalVariables|SetlowDis (Transformation|GetDistanceTo _array_element self))
      (LocalVariables|SetlowIndex _array_index)))
  (Variables|Default|SettargetBall (Utilities|Array|Get(acopy) _outactors (LocalVariables|GetlowIndex))))

(fn CheckBall
  (if (Utilities|IsValid (Variables|Default|GettargetBall))
    (if (Variables|/Game/BluePrints/Core-Gameplay/Dodgeballs/DodgeBall.DodgeBall_C|GetIsCarried (Variables|Default|GettargetBall))
      (return false)
      (else
        (return true)))
    (else
      (return false))))