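; Networking game mode for a single-round sudden death tiebreak between the players sharing the highest score.
; SetUpClients spawns data actors, sets up UI and camera through the game state, then runs pre-round and starts the round after a five-second delay.
; SpawnPlayerPawns finds the top score, spawns pawns only for players matching it and collects the rest for podiums, though SetPodiums is still an empty stub.
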(event EventBeginPlay
  (|CallParentFunction))

(event EventTick
  (params (DeltaSeconds :type Float%20%28single-precision%29))
  (|CallParentFunction 0.0))

(event EventSpawnPlayerPawns
  ;[1 1 1] FindHighScore
  (bind _outactors (Actor|GetAllActorsOfClass "/Script/Rebound_4_12.R_PlayerState"))
  (for _array_element _outactors
    (if (> (Variables|/Script/Rebound_4_12.R_PlayerState|GetPlayerScore _array_element) (Variables|Default|GetHighScore))
      (Variables|Default|SetHighScore (Variables|/Script/Rebound_4_12.R_PlayerState|GetPlayerScore _array_element))))
  ;[1 1 1] spawn pawns and set up podiums
  (for _array_element_2 _outactors
    (if (== (Variables|/Script/Rebound_4_12.R_PlayerState|GetPlayerScore _array_element_2) (Variables|Default|GetHighScore))
      (bind _asnetworking_player_controller (Utilities|Casting|CastToNetworkingPlayerController (Game|GetInstigatorController _array_element_2)))
      (Default|SpawnPawn _asnetworking_player_controller (Transformation|GetActorTransform (Class|GameMode|FindPlayerStart (Game|GetInstigatorController _array_element_2))) (Variables|Default|GetMainPlayerPawn))
      (else
        (Utilities|Array|Add (Variables|Default|GetpodiumPlayer) _array_element_2))))
  ;[1 1 1] pre round set up
  (bind _outactors_2 (Actor|GetAllActorsOfClass "/Game/BluePrints/Core-Gameplay/Characters/ReboundPlayerCharacter.ReboundPlayerCharacter_C"))
  (bind _output_get (Variables|Default|SetPlayerPawns _outactors_2))
  (Variables|Default|SetcurrentPlayers (- (Utilities|Array|Length _output_get) 1))
  (Utilities|FlowControl|DoOnce false
    (:Completed
      (CallFunction|SetPodiums))))

(event EventSetUpClients
  (CallFunction|SpawnDataActors)
  ;[0.03484 0.4387 1] UI and camera
  (bind _asmain_networking_game_state (Utilities|Casting|CastToMainNetworkingGameState (Game|GetGameState)))
  (Default|GetPlayerStates _asmain_networking_game_state)
  (Default|SpawnUI _asmain_networking_game_state)
  (Default|SetUpCamera _asmain_networking_game_state)
  (CallFunction|BindEvents)
  (Utilities|Casting|CastToPersistentData (Game|GetGameInstance))
  ;[1 0 0.7984] moved update Scors to player state. and rounds WILL be moved to Game State
  (Variables|Default|SetMaxRounds 1)
  (Default|CallStartGame)
  (Default|CallPreRound)
  ;[0 1 0.02804] start 5 second count down
  (Development|PrintString "start timer")
  (Utilities|FlowControl|Delay 5.0)
  (Default|CallStartRound)
  (Development|PrintString "end timer"))

(fn ConstructionScript
  (|CallParentFunction))

(fn SetPodiums)