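; Game mode for the networked podium screen that shows players ranked by score.
; On the authority, it polls until no players are still travelling, then has the game state set up the camera and spawn UI.
; It copies PlayerState scores, hides all podiums through PodiumSetUp, then repeatedly takes the highest remaining score to set up each podium with that player's character, marking used scores as -1.
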(event Custom|waitForPlayers
  ;[1 1 1] waiting for players
  (Networking|SwitchHasAuthority
    (:Authority
      (if (> (Variables|Default|GetNumTravellingPlayers) 0)
        (Utilities|FlowControl|Delay 0.2)
        (CallFunction|WaitforPlayers)
        (Development|PrintString (Utilities|String|BuildString(Integer) "" "waiting for " (Variables|Default|GetNumTravellingPlayers) " players to load"))
        (else
          (Utilities|FlowControl|Delay 0.2)
          (CallFunction|SetUpClients))))))

(event Custom|setUpClients
  (Development|PrintString "set up clients" true true "(R=0.000000,G=0.660000,B=1.000000,A=1.000000)" 2e+01)
  (bind _asnetworking_podium_game_state (Utilities|Casting|CastTonetworkingPodiumGameState (Game|GetGameState)))
  (Default|SetUpCamera _asnetworking_podium_game_state)
  ;[1 1 1] TODO
  (Default|SpawnUI _asnetworking_podium_game_state)
  (CallFunction|SetUpPodiums))

(event EventBeginPlay
  ;[1 1 1] begin
  (Utilities|FlowControl|Delay 1.0)
  (CallFunction|WaitforPlayers))

(fn ConstructionScript)

(fn SetUpPodiums
  (bind _scores (LocalVariables|GetScores))
  (bind (_indexofmaxvalue _maxvalue) (Math|Integer|MaxOfIntArray _scores))
  (Development|PrintString "set up podiums" true true "(R=1.000000,G=0.332563,B=0.000000,A=1.000000)" 2e+01)
  ;[1 1 1] check for draw
  (bind _outactors (Actor|GetAllActorsOfClass "/Script/Rebound_4_12.R_PlayerState"))
  (for (_array_element _array_index) _outactors
    (Utilities|Array|SetArrayElem (LocalVariables|GetScores) _array_index (Variables|/Script/Rebound_4_12.R_PlayerState|GetPlayerScore _array_element) true))
  (bind _outactors_2 (Actor|GetAllActorsOfClass "/Game/BluePrints/enviroment/PodiumSetUp.PodiumSetUp_C"))
  (for _array_element_2 (Variables|/Game/BluePrints/enviroment/PodiumSetUp.PodiumSetUp_C|GetPodiums (Utilities|Array|Get(acopy) _outactors_2))
    (Default|MultiHidePodium _array_element_2)
    (Development|PrintString "hide Podiums" true true "(R=0.235331,G=0.000000,B=1.000000,A=1.000000)" 2e+01))
  (for (_ _array_index_2) _outactors
    (Default|MultiSetUpPod (Utilities|Array|Get(acopy) (Variables|/Game/BluePrints/enviroment/PodiumSetUp.PodiumSetUp_C|GetPodiums (Utilities|Array|Get(acopy) _outactors_2)) _array_index_2) _array_index_2 (Variables|/Script/Rebound_4_12.R_PlayerState|GetCusChar (Utilities|Array|Get(acopy) _outactors _indexofmaxvalue)) _maxvalue)
    (Utilities|Array|SetArrayElem (LocalVariables|GetScores) _indexofmaxvalue -1)
    (Development|PrintString "set up podium" true true "(R=1.000000,G=0.000000,B=0.905744,A=1.000000)" 2e+01)))