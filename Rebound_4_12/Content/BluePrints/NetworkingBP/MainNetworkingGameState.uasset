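; Game state for the networked game that manages round UI and relays round start and end events.
; On BeginPlay it binds to NetworkingGameMode's round events, toggling the UI through Rep-prefixed events and calling CallStartRound or CallEndRound.
; A spawn event creates the in-game, end-round and start-game widgets.
; Authority-only events gather player states and trigger camera setup on every NetworkingPlayerController.
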(event Custom|getPlayerStates
  ;[1 1 1] getplayerStates
  (Networking|SwitchHasAuthority
    (:Authority
      (bind _outactors (Actor|GetAllActorsOfClass "/Script/Rebound_4_12.R_PlayerState"))
      (Variables|Default|SetplayerStates _outactors))))

(event Custom|spawnUI
  ;[1 1 1] UI on player Controller
  (bind _returnvalue (UserInterface|CreateWidget "/Game/UI/InGame/InGameUI.InGameUI_C"))
  (bind _returnvalue_2 (UserInterface|CreateWidget "/Game/UI/InGame/EndRound.EndRound_C"))
  (bind _returnvalue_3 (UserInterface|CreateWidget "/Game/UI/InGame/StartGame.StartGame_C"))
  (bind _output_get (Variables|LocalUI|SetinGame _returnvalue))
  (bind _output_get_2 (Variables|LocalUI|SetEndRoundUI _returnvalue_2))
  (bind _output_get_3 (Variables|LocalUI|SetstartGame _returnvalue_3))
  (UserInterface|Viewport|AddtoViewport _output_get 0)
  (Widget|SetVisibility _output_get_2 "Hidden"))

(event Custom|hideUI
  (CallFunction|RepHideUI)
  (Default|CallStartRound))

(event Custom|showUI
  (CallFunction|RepShowUI)
  (Default|CallEndRound))

(event Custom|SetUpCamera
  ;[1 1 1] call the set up cameras per controller
  (Networking|SwitchHasAuthority
    (:Authority
      (bind _outactors (Actor|GetAllActorsOfClass "/Game/BluePrints/NetworkingBP/NetworkingPlayerController.NetworkingPlayerController_C"))
      (for _array_element _outactors
        (Default|SetUpCam _array_element)))))

(event Custom|RepHideUI
  (Widget|SetVisibility (Variables|LocalUI|GetinGame) "Hidden")
  (Widget|SetVisibility (Variables|LocalUI|GetEndRoundUI) "Hidden")
  (Widget|SetVisibility (Variables|LocalUI|GetstartGame) "Hidden"))

(event Custom|RepShowUI
  (Widget|SetVisibility (Variables|LocalUI|GetinGame) "Visible")
  (Widget|SetVisibility (Variables|LocalUI|GetEndRoundUI) "Visible"))

(event EventBeginPlay
  (bind _asnetworking_game_mode (Utilities|Casting|CastToNetworkingGameMode (Game|GetGameMode)))
  (EventDispatchers|BindEventtoStartRound _asnetworking_game_mode (delegate Custom|hideUI))
  (EventDispatchers|BindEventtoEndRound _asnetworking_game_mode (delegate Custom|showUI)))

(fn ConstructionScript)