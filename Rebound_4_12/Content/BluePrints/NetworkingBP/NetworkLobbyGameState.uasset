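; Lobby GameState Blueprint that shows the network lobby menu on each machine and hides it for the host when the server moves.
; On BeginPlay it creates the NetworkMenuUI widget, configures it as host or client by authority, and adds it to the viewport.
; It then binds to the ReboundNetworkLobbyMode move-server event, which removes the widget on authority only.
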(event Custom|moveServer
  (Networking|SwitchHasAuthority
    (:Authority
      (CallFunction|HideUI))))

(event Custom|hideUI
  (Widget|RemovefromParent (Variables|Default|GetlobbyUI)))

(event EventBeginPlay
  ;[1 1 1] UI
  (bind _returnvalue (UserInterface|CreateWidget "/Game/UI/MainMenu/NetworkMenuUI.NetworkMenuUI_C"))
  (bind _output_get (Variables|Default|SetlobbyUI _returnvalue))
  (Networking|SwitchHasAuthority
    (:Authority
      (Default|SetUpHost _output_get))
    (:Remote
      (Default|SetUpClient _output_get)))
  (UserInterface|Viewport|AddtoViewport _output_get 0)
  (bind _asrebound_network_lobby_mode (Utilities|Casting|CastToReboundNetworkLobbyMode (Game|GetGameMode)))
  (EventDispatchers|BindEventtoMoveServer _asrebound_network_lobby_mode (delegate Custom|moveServer)))

(fn ConstructionScript)