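; Player controller for the network lobby that gives each player a pawn, lets them cycle character meshes and drives the lobby UI.
; Setup spawns and possesses a NetworkLobbyPawn at the game mode's player start, points the view at the MainMenuBP camera, then refreshes all characters.
; Mesh changes are stored in R_PlayerState and applied to the pawn.
; UI inputs forward to the game state's LobbyUI, cached on first Tick.
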(event Custom|RepFirstTimeSetUp
  (CallFunction|ServerSetUp)
  (CallFunction|UpdateCharacter)
  (bind _asrebound_network_lobby_mode (Utilities|Casting|CastToReboundNetworkLobbyMode (Game|GetGameMode)))
  (Default|UpdateAllCharacters _asrebound_network_lobby_mode))

(event Custom|ClientSetUp
  (Variables|Default|SetbShowMouseCursor true)
  (Variables|Default|SetbEnableMouseOverEvents true)
  (bind _outactors (Actor|GetAllActorsOfClass "/Game/UI/MainMenu/MainMenuBP.MainMenuBP_C"))
  (Game|Player|SetViewTargetwithBlend (Variables|/Game/UI/MainMenu/MainMenuBP.MainMenuBP_C|Getcamera (Utilities|Array|Get(acopy) _outactors)) 0.0 "VTBlend_Linear" 0.0 false)
  (Development|PrintString "player Set up" true true "(R=1.000000,G=0.338233,B=0.000000,A=1.000000)" 5.0))

(event Custom|RepUpdateCharacter
  (params (customChar :type R%20S%20Custom%20Character%20Structure))
  (bind _output_get (Variables|/Script/Rebound_4_12.R_PlayerState|SetCusChar (Variables|Default|GetreboundPlayerState) customChar))
  (Default|RepSetUpChar (Variables|Default|GetlobbyPawn) _output_get))

(event Custom|ServerSetUp
  (bind _self self)
  (bind _asrebound_network_lobby_mode (Utilities|Casting|CastToReboundNetworkLobbyMode (Game|GetGameMode)))
  (bind _transform (Default|GetPlayerStart _asrebound_network_lobby_mode _self))
  (bind _returnvalue (Game|SpawnActorfromClass "/Game/BluePrints/NetworkingBP/NetworkLobbyPawn.NetworkLobbyPawn_C" _transform "Undefined" _self 0))
  (Pawn|Possess _returnvalue)
  (Development|PrintString "set up pawn" true true "(R=1.000000,G=0.110636,B=0.000000,A=1.000000)" 5.0)
  (bind _asr_player_state (Utilities|Casting|CastToR_PlayerState (Variables|GetPlayerState)))
  (Variables|Default|SetreboundPlayerState _asr_player_state)
  (bind _asnetwork_lobby_pawn (Utilities|Casting|CastToNetworkLobbyPawn (Pawn|GetControlledPawn)))
  (Variables|Default|SetlobbyPawn _asnetwork_lobby_pawn)
  (CallFunction|ClientSetUp))

(event Custom|UpdateCharacter
  (Default|RepSetUpChar (Variables|Default|GetlobbyPawn) (Variables|/Script/Rebound_4_12.R_PlayerState|GetCusChar (Variables|Default|GetreboundPlayerState))))

(event EventTick
  (params (DeltaSeconds :type Float%20%28single-precision%29))
  (Utilities|FlowControl|DoOnce false
    (:Completed
      (bind _asnetwork_lobby_game_state (Utilities|Casting|CastToNetworkLobbyGameState (Game|GetGameState)))
      (Variables|Default|SetUI (Variables|/Game/BluePrints/NetworkingBP/NetworkLobbyGameState.NetworkLobbyGameState_C|GetlobbyUI _asnetwork_lobby_game_state)))))

(event Input|ActionEvents|InputActionPrevMesh
  (params (Key :type Key%20Structure :default "AnyKey"))
  (:Pressed
    (bind _result (Math|Integer|DecrementInt (Variables|Default|GetMeshID))
      (:%20%20
        (if (== _result -1)
          (Variables|Default|SetMeshID (- (Utilities|Array|Length (Variables|Default|GetMesh)) 1)))
        (CallFunction|RepUpdateCharacter (Utilities|Struct|MakeR_S_CustomCharacter (.charcolour (Variables|/Script/Rebound_4_12.R_PlayerState|GetCusChar (Variables|Default|GetreboundPlayerState))) (Utilities|Array|Get(acopy) (Variables|Default|GetMesh) (Variables|Default|GetMeshID)) (Utilities|Enum|ByteToEnumER_E_PlayerMesh (Math|Conversions|ToByte(Integer) (Variables|Default|GetMeshID))) (Utilities|Array|Get(acopy) (Variables|Default|GetMat) (Variables|Default|GetMeshID))))))))

(event Input|ActionEvents|InputActionSelectUI
  (params (Key :type Key%20Structure :default "AnyKey"))
  (:Pressed
    (Default|SelectUI (Variables|Default|GetUI))))

(event Input|ActionEvents|InputActionUpUI
  (params (Key :type Key%20Structure :default "AnyKey"))
  (:Pressed
    (Default|UpUI (Variables|Default|GetUI))))

(event Input|ActionEvents|InputActionDownUI
  (params (Key :type Key%20Structure :default "AnyKey"))
  (:Pressed
    (Default|DownUI (Variables|Default|GetUI))))

(event Input|ActionEvents|InputActionswapUIleft
  (params (Key :type Key%20Structure :default "AnyKey"))
  (:Pressed
    (Default|MoveFocusLeft (Variables|Default|GetUI))))

(event Input|ActionEvents|InputActionswapUIRight
  (params (Key :type Key%20Structure :default "AnyKey"))
  (:Pressed
    (Default|MoveFocusRight (Variables|Default|GetUI))))

(event Input|ActionEvents|InputActionNextMesh
  (params (Key :type Key%20Structure :default "AnyKey"))
  (:Released
    (bind _result (Math|Integer|IncrementInt (Variables|Default|GetMeshID))
      (:%20%20
        (if (== _result (Utilities|Array|Length (Variables|Default|GetMesh)))
          (Variables|Default|SetMeshID 0))
        (CallFunction|RepUpdateCharacter (Utilities|Struct|MakeR_S_CustomCharacter (.charcolour (Variables|/Script/Rebound_4_12.R_PlayerState|GetCusChar (Variables|Default|GetreboundPlayerState))) (Utilities|Array|Get(acopy) (Variables|Default|GetMesh) (Variables|Default|GetMeshID)) (Utilities|Enum|ByteToEnumER_E_PlayerMesh (Math|Conversions|ToByte(Integer) (Variables|Default|GetMeshID))) (Utilities|Array|Get(acopy) (Variables|Default|GetMat) (Variables|Default|GetMeshID))))))))

(event Input|ActionEvents|InputActionExit
  (params (Key :type Key%20Structure :default "AnyKey")))

(fn ConstructionScript)