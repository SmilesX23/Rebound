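; Game mode for the Rebound multiplayer lobby, handling player slots, level playlist and match launch.
; On login it assigns each player a number and starting colour from shared pools, returning both on logout; player number also selects the spawn point.
; It can fill the PersistentData playlist with random level and mutator picks from a spawned LobbyLevelData.
; PlayGame flags data loading, then seamlessly server-travels to the first playlist level.
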(event Custom|PlayGame
  (Networking|SwitchHasAuthority
    (:Authority
      (bind _aspersistent_data (Utilities|Casting|CastToPersistentData (Game|GetGameInstance)))
      (Variables|/Game/BluePrints/data/PersistentData.PersistentData_C|SetloadData _aspersistent_data true)
      (Variables|/Game/BluePrints/data/PersistentData.PersistentData_C|SetplaylistPos _aspersistent_data 0)
      (Variables|Default|SetbUseSeamlessTravel true)
      (if (!= (Utilities|Array|Length (Variables|/Game/BluePrints/data/PersistentData.PersistentData_C|Getplaylist _aspersistent_data)) 0)
        (Default|CallMoveServer)
        (Utilities|FlowControl|Delay 0.2)
        ;[1 1 1] move server
        (Development|ExecuteConsoleCommand (Utilities|String|Append "servertravel " (Utilities|String|ToString(Name) (.levelname (Utilities|Array|Get(acopy) (Variables|/Game/BluePrints/data/PersistentData.PersistentData_C|Getplaylist _aspersistent_data))))))
        (else
          (Development|PrintString "nothing in playlist"))))))

(event Custom|UpdateAllCharacters
  (bind _outactors (Actor|GetAllActorsOfClass "/Game/BluePrints/NetworkingBP/NetworkLobbyController.NetworkLobbyController_C"))
  (for _array_element _outactors
    (Default|UpdateCharacter _array_element)))

(event EventBeginPlay
  ;[1 1 1] server start
  (bind _returnvalue (Game|SpawnActorfromClass "/Game/BluePrints/NetworkingBP/LobbyLevelData.LobbyLevelData_C" (Math|Transform|MakeTransform "0, 0, 0" "0, 0, 0" "1,1,1") "Undefined" 0 0))
  (Variables|Default|SetLobbyLevelData _returnvalue))

(event EventPostLogin
  (params (NewPlayer :type Player%20Controller%20Object%20Reference))
  (bind _playernums (Variables|Default|GetPlayerNums))
  (bind _startingcolours (Variables|Default|GetStartingColours))
  (bind _item (Utilities|Array|Get(acopy) _startingcolours))
  ;[1 1 1] player joins
  (Development|PrintString "player joined" true true "(R=0.224048,G=1.000000,B=0.000000,A=1.000000)" 2e+01)
  (bind _asnetwork_lobby_controller (Utilities|Casting|CastToNetworkLobbyController NewPlayer))
  (bind _asr_player_state (Utilities|Casting|CastToR_PlayerState (Variables|/Script/Engine.Controller|GetPlayerState _asnetwork_lobby_controller)))
  (bind _output_get (Variables|/Script/Rebound_4_12.R_PlayerState|SetPlayerNum _asr_player_state (Utilities|Array|Get(acopy) _playernums)))
  (Utilities|Array|RemoveItem _playernums _output_get)
  (Variables|/Script/Rebound_4_12.R_PlayerState|SetCusChar _asr_player_state (Utilities|Struct|MakeR_S_CustomCharacter _item "/Game/Art/Character/Character_new/Character_rigged.Character_rigged" "PM_Male" "/Game/Art/Character/Character_new/playerColourInstance.playerColourInstance"))
  (Utilities|Array|RemoveItem _startingcolours _item)
  (Default|RepFirstTimeSetUp _asnetwork_lobby_controller))

(event EventOnLogout
  (params (ExitingController :type Controller%20Object%20Reference))
  ;[1 1 1] player leaves
  (Development|PrintString "player left" true true "(R=0.224048,G=1.000000,B=0.000000,A=1.000000)" 5.0)
  (bind _asr_player_state (Utilities|Casting|CastToR_PlayerState (Variables|/Script/Engine.Controller|GetPlayerState ExitingController)))
  (Utilities|Array|Add (Variables|Default|GetPlayerNums) (Variables|/Script/Rebound_4_12.R_PlayerState|GetPlayerNum _asr_player_state))
  (Utilities|Array|Add (Variables|Default|GetStartingColours) (.charcolour (Variables|/Script/Rebound_4_12.R_PlayerState|GetCusChar _asr_player_state))))

(fn ConstructionScript)

(fn GetPlayerStart
  (params (player :type Player%20Controller%20Object%20Reference))
  (bind _asr_player_state (Utilities|Casting|CastToR_PlayerState (Variables|/Script/Engine.Controller|GetPlayerState player))
    (:then
      (bind _outactors (Actor|GetAllActorsOfClass "/Script/Engine.PlayerStart"))
      (return (Transformation|GetActorTransform (Utilities|Array|Get(acopy) _outactors (Variables|/Script/Rebound_4_12.R_PlayerState|GetPlayerNum _asr_player_state)))))
    (:CastFailed
      (bind _outactors_2 (Actor|GetAllActorsOfClass "/Script/Engine.PlayerStart"))
      (return (Transformation|GetActorTransform (Utilities|Array|Get(acopy) _outactors_2 1))))))

(fn PlaylistAddRandom
  (params (NoToAdd :type Integer))
  (bind _lobbyleveldata (Variables|Default|GetLobbyLevelData))
  (bind _levelnames (Variables|/Game/BluePrints/NetworkingBP/LobbyLevelData.LobbyLevelData_C|GetLevelNames _lobbyleveldata))
  (bind _mutators (Variables|/Game/BluePrints/NetworkingBP/LobbyLevelData.LobbyLevelData_C|GetMutators _lobbyleveldata))
  (bind _aspersistent_data (Utilities|Casting|CastToPersistentData (Game|GetGameInstance)))
  (Utilities|Array|Clear (Variables|/Game/BluePrints/data/PersistentData.PersistentData_C|Getplaylist _aspersistent_data))
  (for _index (range 0 NoToAdd)
    (Utilities|Array|Add (Variables|/Game/BluePrints/data/PersistentData.PersistentData_C|Getplaylist _aspersistent_data) (Utilities|Struct|MakeR_S_LevelStruct (Utilities|Array|Get(acopy) _levelnames (Math|Random|RandomIntegerinRange 0 (- (Utilities|Array|Length _levelnames) 1))) 5 (Utilities|Array|Get(acopy) _mutators (Math|Random|RandomIntegerinRange 0 (- (Utilities|Array|Length _mutators) 1)))))))