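; Killzone actor for Rebound that kills players and despawns dodgeballs that overlap its Cube component.
; On overlap it spawns an explosion at its own location, then handles the other actor by type.
; Players drop any carried ball, which BallData despawns, and are reported to ReboundGameMode as died.
; Loose dodgeballs are despawned through the first BallData actor found in the level.
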(event Custom|OnComponentBeginOverlap_Event_0
  (params (OverlappedComponent :type Primitive%20Component%20Object%20Reference) (OtherActor :type Actor%20Object%20Reference) (OtherComp :type Primitive%20Component%20Object%20Reference) (OtherBodyIndex :type Integer) (bFromSweep :type Boolean) (SweepResult :type Hit%20Result%20Structure%20%28by%20ref%29))
  (CallFunction|OverlapCheck OtherActor))

(event EventBeginPlay
  (Collision|AssignOnComponentBeginOverlap (Variables|Default|GetCube) (delegate Custom|OnComponentBeginOverlap_Event_0)))

(fn ConstructionScript)

(fn OverlapCheck
  (params (Other :type Actor%20Object%20Reference))
  (Effects|SpawnEmitteratLocation "/Game/Art/Particles/Explosion.Explosion" (Transformation|GetActorLocation))
  (if (not (Game|IsActorBeingDestroyed Other))
    (bind _asrebound_game_mode (Utilities|Casting|CastToReboundGameMode (Game|GetGameMode)))
    (bind _asrebound_player_character (Utilities|Casting|CastToReboundPlayerCharacter Other)
      (:then
        (if (Variables|/Game/BluePrints/Core-Gameplay/Characters/ReboundPlayerCharacter.ReboundPlayerCharacter_C|GetIsCarryingDodgeball _asrebound_player_character)
          (Default|DropBall _asrebound_player_character true)
          (bind _outactors (Actor|GetAllActorsOfClass "/Game/BluePrints/data/BallData.BallData_C"))
          (if (not (< (Utilities|Array|Length _outactors) 1))
            (Default|DespawnABall (Utilities|Array|Get(acopy) _outactors) (Variables|/Game/BluePrints/Core-Gameplay/Characters/ReboundPlayerCharacter.ReboundPlayerCharacter_C|GetCarriedDodgeBall _asrebound_player_character))
            (Default|PlayerDied _asrebound_game_mode 0 0 false _asrebound_player_character :!label _label))
          (else
            (goto _label))))
      (:CastFailed
        (bind _asdodge_ball (Utilities|Casting|CastToDodgeBall Other))
        (bind _outactors_2 (Actor|GetAllActorsOfClass "/Game/BluePrints/data/BallData.BallData_C"))
        (if (not (< (Utilities|Array|Length _outactors_2) 1))
          (Default|DespawnABall (Utilities|Array|Get(acopy) _outactors_2) _asdodge_ball))))))