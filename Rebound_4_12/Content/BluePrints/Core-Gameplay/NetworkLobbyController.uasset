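; Player controller for the network lobby that sets up the player's menu UI, camera view and pawn on BeginPlay.
; It creates and displays the NetworkMenuUI widget, stores it as the chat UI, enables the mouse cursor and switches the view to the main menu actor's camera.
; It then asks the ReboundNetworkLobbyMode game mode for a player start, spawns a NetworkLobbyPawn there and possesses it, printing debug messages along the way.
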(event EventBeginPlay
  (bind _self self)
  (bind _returnvalue (UserInterface|CreateWidget "/Game/UI/MainMenu/NetworkMenuUI.NetworkMenuUI_C"))
  (Variables|Default|SetChatUI _returnvalue)
  (UserInterface|Viewport|AddtoViewport _returnvalue 0)
  (Variables|Default|SetbShowMouseCursor true)
  (Variables|Default|SetbEnableMouseOverEvents true)
  (bind _outactors (Actor|GetAllActorsOfClass "/Game/UI/MainMenu/MainMenuBP.MainMenuBP_C"))
  (Game|Player|SetViewTargetwithBlend (Variables|/Game/UI/MainMenu/MainMenuBP.MainMenuBP_C|Getcamera (Utilities|Array|Get(acopy) _outactors)) 0.0 "VTBlend_Linear" 0.0 false)
  (Development|PrintString "player Set up" true true "(R=1.000000,G=0.338233,B=0.000000,A=1.000000)" 5.0)
  (bind _asrebound_network_lobby_mode (Utilities|Casting|CastToReboundNetworkLobbyMode (Game|GetGameMode)))
  (bind _transform (Default|GetPlayerStart _asrebound_network_lobby_mode _self))
  (bind _returnvalue_2 (Game|SpawnActorfromClass "/Game/BluePrints/Core-Gameplay/NetworkLobbyPawn.NetworkLobbyPawn_C" _transform "Undefined" _self 0))
  (Pawn|Possess _returnvalue_2)
  (Development|PrintString "set up pawn" true true "(R=1.000000,G=0.110636,B=0.000000,A=1.000000)" 5.0))

(event EventTick
  (params (DeltaSeconds :type Float%20%28single-precision%29)))

(fn ConstructionScript)