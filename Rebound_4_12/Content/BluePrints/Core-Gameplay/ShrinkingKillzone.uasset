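; Shrinking killzone for Rebound rounds that closes in on the arena and eliminates players it touches.
; Game mode round start arms a timer that reveals four boundary pieces, slides them on Tick, plays killzone audio and raises all battle music layers.
; Overlaps report player deaths to the game mode and despawn dodgeballs, carried or loose, through BallData.
; Round end restores saved positions, hides the zone and clears the timer.
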(event OnComponentBeginOverlap(B1)
  (params (OverlappedComponent :type Primitive%20Component%20Object%20Reference) (OtherActor :type Actor%20Object%20Reference) (OtherComp :type Primitive%20Component%20Object%20Reference) (OtherBodyIndex :type Integer) (bFromSweep :type Boolean) (SweepResult :type Hit%20Result%20Structure%20%28by%20ref%29))
  (CallFunction|OverlapCheck OtherActor))

(event OnComponentBeginOverlap(B4)
  (params (OverlappedComponent :type Primitive%20Component%20Object%20Reference) (OtherActor :type Actor%20Object%20Reference) (OtherComp :type Primitive%20Component%20Object%20Reference) (OtherBodyIndex :type Integer) (bFromSweep :type Boolean) (SweepResult :type Hit%20Result%20Structure%20%28by%20ref%29))
  (CallFunction|OverlapCheck OtherActor))

(event OnComponentBeginOverlap(B3)
  (params (OverlappedComponent :type Primitive%20Component%20Object%20Reference) (OtherActor :type Actor%20Object%20Reference) (OtherComp :type Primitive%20Component%20Object%20Reference) (OtherBodyIndex :type Integer) (bFromSweep :type Boolean) (SweepResult :type Hit%20Result%20Structure%20%28by%20ref%29))
  (CallFunction|OverlapCheck OtherActor))

(event OnComponentBeginOverlap(B2)
  (params (OverlappedComponent :type Primitive%20Component%20Object%20Reference) (OtherActor :type Actor%20Object%20Reference) (OtherComp :type Primitive%20Component%20Object%20Reference) (OtherBodyIndex :type Integer) (bFromSweep :type Boolean) (SweepResult :type Hit%20Result%20Structure%20%28by%20ref%29))
  (CallFunction|OverlapCheck OtherActor))

(event Custom|TimerStart
  (bind _returnvalue (Utilities|Time|SetTimerbyEvent (delegate Custom|Shrink) (Variables|Default|GetTimerToShrink)))
  (Variables|Default|SetTimerHandle _returnvalue))

(event Custom|Reset
  (bind _timerhandle (Variables|Default|GetTimerHandle))
  (bind _startpositions (Variables|Default|GetStartPositions))
  (Variables|Default|SetBeginShrink false)
  (Transformation|SetWorldLocation (Variables|Default|GetB1) (Utilities|Array|Get(acopy) _startpositions) false true)
  (Transformation|SetWorldLocation (Variables|Default|GetB2) (Utilities|Array|Get(acopy) _startpositions 1) false true)
  (Transformation|SetWorldLocation (Variables|Default|GetB3) (Utilities|Array|Get(acopy) _startpositions 2) false true)
  (Transformation|SetWorldLocation (Variables|Default|GetB4) (Utilities|Array|Get(acopy) _startpositions 3) false true)
  (Rendering|SetVisibility (Variables|Default|GetDefaultSceneRoot) false true)
  (Audio|Components|Audio|Stop (Variables|Default|GetKillzone))
  (if (Utilities|Time|IsValidTimerHandle _timerhandle)
    (Utilities|Time|ClearandInvalidateTimerbyHandle _timerhandle)))

(event Custom|Shrink
  (Variables|Default|SetBeginShrink true)
  (Rendering|SetVisibility (Variables|Default|GetB1) true false)
  (Rendering|SetVisibility (Variables|Default|GetB2) true false)
  (Rendering|SetVisibility (Variables|Default|GetB3) true false)
  (Rendering|SetVisibility (Variables|Default|GetB4) true false)
  (Audio|Components|Audio|Play (Variables|Default|GetKillzone) 0.0)
  (bind _asrebound_game_mode (Utilities|Casting|CastToReboundGameMode (Game|GetGameMode)))
  (Audio|Parameter|SetFloatParameter (Variables|/Game/BluePrints/Gamemodes/ReboundGameMode.ReboundGameMode_C|GetBattleMusic _asrebound_game_mode) "LowLayer" 1.0 :!class /Script/Engine.AudioComponent)
  (Audio|Parameter|SetFloatParameter (Variables|/Game/BluePrints/Gamemodes/ReboundGameMode.ReboundGameMode_C|GetBattleMusic _asrebound_game_mode) "MediumLayer" 1.0 :!class /Script/Engine.AudioComponent)
  (Audio|Parameter|SetFloatParameter (Variables|/Game/BluePrints/Gamemodes/ReboundGameMode.ReboundGameMode_C|GetBattleMusic _asrebound_game_mode) "HighLayer" 1.0 :!class /Script/Engine.AudioComponent))

(event EventTick
  (params (DeltaSeconds :type Float%20%28single-precision%29))
  (bind _shrinkspeed (Variables|Default|GetShrinkSpeed))
  (bind _returnvalue (* DeltaSeconds _shrinkspeed))
  (bind _returnvalue_2 (* _returnvalue -1.0))
  (if (Variables|Default|GetBeginShrink)
    (Transformation|AddLocalOffset (Variables|Default|GetB1) (Math|Vector|MakeVector _returnvalue_2 0.0 0.0) true false)
    (Transformation|AddLocalOffset (Variables|Default|GetB2) (Math|Vector|MakeVector _returnvalue 0.0 0.0) true false)
    (Transformation|AddLocalOffset (Variables|Default|GetB3) (Math|Vector|MakeVector 0.0 _returnvalue 0.0) true false)
    (Transformation|AddLocalOffset (Variables|Default|GetB4) (Math|Vector|MakeVector 0.0 _returnvalue_2 0.0) true false)))

(event EventBeginPlay
  (bind _startpositions (Variables|Default|GetStartPositions))
  (bind _asrebound_game_mode (Utilities|Casting|CastToReboundGameMode (Game|GetGameMode)))
  (EventDispatchers|BindEventtoStartRound _asrebound_game_mode (delegate Custom|TimerStart))
  (EventDispatchers|BindEventtoEndRound _asrebound_game_mode (delegate Custom|Reset))
  (Rendering|SetVisibility (Variables|Default|GetDefaultSceneRoot) false true)
  (Utilities|Array|SetArrayElem _startpositions 0 (Transformation|GetWorldLocation (Variables|Default|GetB1)) true)
  (Utilities|Array|SetArrayElem _startpositions 1 (Transformation|GetWorldLocation (Variables|Default|GetB2)) true)
  (Utilities|Array|SetArrayElem _startpositions 2 (Transformation|GetWorldLocation (Variables|Default|GetB3)) true)
  (Utilities|Array|SetArrayElem _startpositions 3 (Transformation|GetWorldLocation (Variables|Default|GetB4)) true))

(fn ConstructionScript)

(fn OverlapCheck
  (params (Other :type Actor%20Object%20Reference))
  (if (not (Game|IsActorBeingDestroyed Other))
    (bind _asrebound_game_mode (Utilities|Casting|CastToReboundGameMode (Game|GetGameMode)))
    (bind _asrebound_player_character (Utilities|Casting|CastToReboundPlayerCharacter Other)
      (:then
        (if (Variables|/Game/BluePrints/Core-Gameplay/Characters/ReboundPlayerCharacter.ReboundPlayerCharacter_C|GetIsCarryingDodgeball _asrebound_player_character)
          (Default|DropBall _asrebound_player_character true)
          (bind _outactors (Actor|GetAllActorsOfClass "/Game/BluePrints/data/BallData.BallData_C"))
          (if (not (< (Utilities|Array|Length _outactors) 1))
            (Default|DespawnABall (Utilities|Array|Get(acopy) _outactors) (Variables|/Game/BluePrints/Core-Gameplay/Characters/ReboundPlayerCharacter.ReboundPlayerCharacter_C|GetCarriedDodgeBall _asrebound_player_character))
            (Default|PlayerDied _asrebound_game_mode 0 0 false _asrebound_player_character :!label _label))
          (else
            (goto _label))))
      (:CastFailed
        (bind _asdodge_ball (Utilities|Casting|CastToDodgeBall Other))
        (bind _outactors_2 (Actor|GetAllActorsOfClass "/Game/BluePrints/data/BallData.BallData_C"))
        (if (not (< (Utilities|Array|Length _outactors_2) 1))
          (Default|DespawnABall (Utilities|Array|Get(acopy) _outactors_2) _asdodge_ball))))))