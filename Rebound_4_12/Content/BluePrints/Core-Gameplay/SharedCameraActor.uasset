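; Shared camera that frames all living player characters, easing toward their average position unless set static.
; Zoom lerps between two offsets through a curve of player spread relative to a maximum from PlayerStart spacing or an override.
; NetworkingGameMode events refresh the tracked players, shake the camera on death and post-round, and trigger timeline-driven slow motion at round end.
; A dynamic post-process material applies the saved gamma setting every tick.
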(event Custom|PlayerRemoved
  (CallFunction|UpdateActivePlayers)
  (Camera|PlayWorldCameraShake "/Game/BluePrints/Core-Gameplay/PlayerDeathCamShake.PlayerDeathCamShake_C" (Transformation|GetActorLocation) 1e+02 1e+02))

(event Custom|StartRoundCall
  (Utilities|Time|SetTimerbyFunctionName self "UpdateActivePlayers" 0.1))

(event Custom|SlowMotionDeath
  (bind _timedialation (Timeline|SloMo PlayFromStart)
    (:Update
      (Utilities|Time|SetGlobalTimeDilation _timedialation))))

(event EventBeginPlay
  (bind _standardmaxdistanceoverride (Variables|Default|GetStandardMaxDistanceOverride))
  (if (> _standardmaxdistanceoverride -1.0)
    (Variables|Default|SetMaxDistance _standardmaxdistanceoverride)
    (else
      (bind _maxdistance (CallFunction|GetMaxDistance "/Script/Engine.PlayerStart"))
      (Variables|Default|SetMaxDistance _maxdistance)))
  (Variables|Default|SetStartingRotation (Transformation|GetWorldRotation (Variables|Default|GetCamera)))
  (Variables|Default|SetStartingPosition (Transformation|GetActorLocation))
  (bind _asnetworking_game_mode (Utilities|Casting|CastToNetworkingGameMode (Game|GetGameMode)))
  (EventDispatchers|BindEventtoPlayerHasDied _asnetworking_game_mode (delegate Custom|PlayerRemoved))
  (EventDispatchers|BindEventtoPreRound _asnetworking_game_mode (delegate Custom|StartRoundCall))
  (EventDispatchers|BindEventtoEndRound _asnetworking_game_mode (delegate Custom|SlowMotionDeath))
  (EventDispatchers|BindEventtoPostRound _asnetworking_game_mode (delegate Custom|PlayerRemoved))
  (CallFunction|ApplyGamma)
  (bind _aspersistent_data (Utilities|Casting|CastToPersistentData (Game|GetGameInstance)))
  (Variables|Default|SetpersisData _aspersistent_data))

(event EventTick
  (params (DeltaSeconds :type Float%20%28single-precision%29))
  (if (not (Variables|Default|GetStatic))
    (bind _maxdistance (CallFunction|GetMaxDistance))
    (bind _updatedoffset (CallFunction|DynamicZoom _maxdistance))
    (bind _output_get (Variables|Default|SetcurrentOffset (Math|Vector|RotateVector _updatedoffset (Math|Rotator|MakeRotator 0.0 0.0 (+ (Variables|Default|GetRotationOffset) (.yaw (Variables|Default|GetStartingRotation)))))))
    (bind _location (CallFunction|AverageLocation _output_get))
    (bind _output_get_2 (Variables|Default|SetCurrentPos _location))
    (Transformation|SetActorLocation (Math|Interpolation|VInterpTo (Transformation|GetActorLocation) _output_get_2 DeltaSeconds (Variables|Default|GetInterpSpeed)) false false))
  (CallFunction|ApplyGamma))

(fn ConstructionScript)

(fn AverageLocation
  (params (Offset :type Vector))
  (bind _activeplayers (Variables|Default|GetActivePlayers))
  (bind _camera (Variables|Default|GetCamera))
  (bind _camera_2 (Variables|Default|GetCamera))
  (bind _returnvalue (Utilities|Array|Length _activeplayers))
  (bind _returnvalue_2 (Transformation|GetWorldRotation _camera_2))
  (for _array_element _activeplayers
    (LocalVariables|SetTotalLocTemp (+ (Transformation|GetActorLocation _array_element) (LocalVariables|GetTotalLocTemp))))
  (if (> _returnvalue 0)
    (bind _output_get (LocalVariables|SetTotalLocTemp (/ (LocalVariables|GetTotalLocTemp) _returnvalue)))
    (Transformation|SetWorldRotation _camera_2 (Math|Interpolation|RInterpTo (Transformation|GetWorldRotation _camera_2) (Math|Rotator|MakeRotator (.roll _returnvalue_2) (.pitch _returnvalue_2) (+ (Variables|Default|GetRotationOffset) (.yaw (Variables|Default|GetStartingRotation)))) (Utilities|Time|GetWorldDeltaSeconds) (Variables|Default|GetInterpSpeed)) false false)
    (return (Math|Vector|MakeVector (.x (+ _output_get Offset)) (.y (+ _output_get Offset)) (+ (.z (+ _output_get Offset)) (.z (Variables|Default|GetStartingPosition)))))
    (else
      (Transformation|SetWorldRotation _camera (Math|Interpolation|RInterpTo (Transformation|GetWorldRotation _camera) (Variables|Default|GetStartingRotation) (Utilities|Time|GetWorldDeltaSeconds) (Variables|Default|GetInterpSpeed)) false false)
      (return (Variables|Default|GetStartingPosition)))))

(fn DynamicZoom
  (params (CurMaxDistance :type Float%20%28single-precision%29))
  (bind _standardoffset (Variables|Default|GetStandardOffset))
  (if (> (Utilities|Array|Length (Variables|Default|GetActivePlayers)) 0)
    (return (Math|Vector|Lerp(Vector) (Variables|Default|GetLowestPositionOffset) _standardoffset (Math|Curves|GetFloatValue (Variables|Default|GetStandardOffsetDistanceCurve) (/ CurMaxDistance (Variables|Default|GetMaxDistance)))))
    (else
      (return _standardoffset))))

(fn GetMaxDistance
  (params (Class :type Actor%20Class%20Reference))
  (bind _activeplayers (Variables|Default|GetActivePlayers))
  (bind _distances (LocalVariables|GetDistances))
  (bind _distances_2 (LocalVariables|GetDistances))
  (if (!= Class 0)
    (bind _outactors (Actor|GetAllActorsOfClass Class))
    (for _array_element _outactors
      (for _array_element_2 _outactors
        (Utilities|Array|Add _distances (Transformation|GetHorizontalDistanceTo _array_element _array_element_2))))
    (return (.MaxValue (Math|Float|MaxOfFloatArray _distances)))
    (else
      (for _array_element_3 _activeplayers
        (for _array_element_4 _activeplayers
          (Utilities|Array|Add _distances_2 (Transformation|GetHorizontalDistanceTo _array_element_3 _array_element_4))))
      (return (.MaxValue (Math|Float|MaxOfFloatArray _distances_2))))))

(fn UpdateActivePlayers
  (Utilities|Array|Clear (Variables|Default|GetActivePlayers))
  (bind _outactors (Actor|GetAllActorsOfClass "/Game/BluePrints/Core-Gameplay/Characters/ReboundPlayerCharacter.ReboundPlayerCharacter_C"))
  (for _array_element _outactors
    (if (not (Game|IsActorBeingDestroyed _array_element))
      (Utilities|Array|AddUnique (Variables|Default|GetActivePlayers) _array_element))))

(fn ApplyGamma
  (Utilities|IsValid (Variables|Default|GetGammaPostProcessMaterial)
    (:Is%20Valid
      _)
    (:Is%20Not%20Valid
      (bind _returnvalue (Rendering|Material|CreateDynamicMaterialInstance "/Game/Art/PostProcessing/Gamma.Gamma" :!class /Script/Engine.KismetMaterialLibrary))
      (bind _output_get (Variables|Default|SetGammaPostProcessMaterial _returnvalue))
      (Rendering|AddorUpdateBlendable (Variables|Default|GetCamera) _output_get 1.0 :!class /Script/Engine.CameraComponent)))
  (bind _aspersistent_data (Utilities|Casting|CastToPersistentData (Game|GetGameInstance)))
  (Rendering|Material|SetScalarParameterValue (Variables|Default|GetGammaPostProcessMaterial) "GammaStrength" (Variables|/Game/BluePrints/data/PersistentData.PersistentData_C|GetGammaCorrection _aspersistent_data) :!class /Script/Engine.MaterialInstanceDynamic))